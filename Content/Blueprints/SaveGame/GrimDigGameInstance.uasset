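; Game instance for GrimDig that owns the persistent save object for player, level and collectible data.
; On init it loads the save slot, or builds a new save seeded from the level and collectible data tables.
; Helpers save the player's inventory, restore it with movement and grid settings while refilling HP, write level data, find levels by name, and wipe the save back to defaults.
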(event EventInit
  (Utilities|FlowControl|Sequence
    (:then_0
      (bind _returnvalue (SaveGame|DoesSaveGameExist (Variables|Default|GetSaveSlotName)))
      (if _returnvalue
        (bind _returnvalue_2 (SaveGame|LoadGamefromSlot (Variables|Default|GetSaveSlotName)))
        (bind _asgrim_dig_save_game_object (Utilities|Casting|CastToGrimDigSaveGameObject _returnvalue_2))
        (Variables|Default|SetSaveGameData _asgrim_dig_save_game_object)
        (else
          (CallFunction|CreateNewSaveData))))))

(fn SavePlayerData
  (bind _savegamedata (Variables|Default|GetSaveGameData))
  (Variables|/Game/Blueprints/SaveGame/GrimDigSaveGameObject.GrimDigSaveGameObject_C|SetInventory _savegamedata (Variables|/Game/Blueprints/Character/GrimDigPawn.GrimDigPawn_C|GetInventory (Variables|Default|GetPlayerPawnRef)))
  (SaveGame|SaveGametoSlot _savegamedata (Variables|Default|GetSaveSlotName)))

(fn LoadPlayerData
  (bind _savegamedata (Variables|Default|GetSaveGameData))
  (bind _playerpawnref (Variables|Default|GetPlayerPawnRef))
  (Variables|/Game/Blueprints/Character/GrimDigPawn.GrimDigPawn_C|SetHP_CurrentInt _playerpawnref (Variables|/Game/Blueprints/Character/GrimDigPawn.GrimDigPawn_C|GetHP_MaxInt _playerpawnref))
  (Variables|/Game/Blueprints/Character/GrimDigPawn.GrimDigPawn_C|SetInventory _playerpawnref (Variables|/Game/Blueprints/SaveGame/GrimDigSaveGameObject.GrimDigSaveGameObject_C|GetInventory _savegamedata))
  (Variables|/Game/Blueprints/Character/GrimDigPawn.GrimDigPawn_C|SetContinousMovementEnabled? _playerpawnref (Variables|/Game/Blueprints/SaveGame/GrimDigSaveGameObject.GrimDigSaveGameObject_C|GetContinous%20Movement _savegamedata))
  (Variables|/Game/Blueprints/Character/GrimDigPawn.GrimDigPawn_C|SetGridEnabled? _playerpawnref (Variables|/Game/Blueprints/SaveGame/GrimDigSaveGameObject.GrimDigSaveGameObject_C|GetGridEnabled _savegamedata)))

(fn ClearSaveData
  (SaveGame|DeleteGameinSlot (Variables|Default|GetSaveSlotName))
  (CallFunction|CreateNewSaveData))

(fn FindLevelOfName
  (params (Name :type Name))
  (bind (_array_element _array_index) (Utilities|Array|ForEachLoopwithBreak (Variables|/Game/Blueprints/SaveGame/GrimDigSaveGameObject.GrimDigSaveGameObject_C|GetLevelData (Variables|Default|GetSaveGameData)) :!label _label)
    (:LoopBody
      (if (Utilities|Name|Equal(Name) (.LevelName (Utilities|Struct|BreakS_LevelInfoData _array_element)) Name)
        (LocalVariables|SetIndexFound _array_index)
        (goto _label Break)))
    (:Completed
      (return (LocalVariables|GetIndexFound)))))

(fn SaveLevelData
  (SaveGame|SaveGametoSlot (Variables|Default|GetSaveGameData) (Variables|Default|GetSaveSlotName)))

(fn CreateNewSaveData
  (bind _returnvalue (SaveGame|CreateSaveGameObject "/Game/Blueprints/SaveGame/GrimDigSaveGameObject.GrimDigSaveGameObject_C"))
  (Variables|Default|SetSaveGameData _returnvalue)
  (bind _outrownames (DataTable|GetDataTableRowNames (Variables|Default|GetLevelDataTableRef)))
  (for (_array_element _array_index) _outrownames
    (bind _returnvalue_2 (Utilities|GetDataTableRow (Variables|Default|GetLevelDataTableRef) _array_element)
      (:then
        (Utilities|Array|Add (Variables|/Game/Blueprints/SaveGame/GrimDigSaveGameObject.GrimDigSaveGameObject_C|GetLevelData (Variables|Default|GetSaveGameData)) (Utilities|Struct|MakeS_LevelInfoData _array_index (.LevelName (Utilities|Struct|BreakS_LevelInfoData _returnvalue_2)) (.LevelInGameName (Utilities|Struct|BreakS_LevelInfoData _returnvalue_2)) (.Story (Utilities|Struct|BreakS_LevelInfoData _returnvalue_2)) (.PreviewImage (Utilities|Struct|BreakS_LevelInfoData _returnvalue_2)) (.Discovered? (Utilities|Struct|BreakS_LevelInfoData _returnvalue_2)) (.Unlocked? (Utilities|Struct|BreakS_LevelInfoData _returnvalue_2)) (.Finished? (Utilities|Struct|BreakS_LevelInfoData _returnvalue_2)) (.BestGoldFound (Utilities|Struct|BreakS_LevelInfoData _returnvalue_2)) (.AllGold (Utilities|Struct|BreakS_LevelInfoData _returnvalue_2)) (.SecretsFound (Utilities|Struct|BreakS_LevelInfoData _returnvalue_2)) (.AllSecrets (Utilities|Struct|BreakS_LevelInfoData _returnvalue_2)) (.UnlockWithGold? (Utilities|Struct|BreakS_LevelInfoData _returnvalue_2)) (.CostToUnlock (Utilities|Struct|BreakS_LevelInfoData _returnvalue_2)) (.Collectible0 (Utilities|Struct|BreakS_LevelInfoData _returnvalue_2)) (.Collectible1 (Utilities|Struct|BreakS_LevelInfoData _returnvalue_2)) (.Collectible2 (Utilities|Struct|BreakS_LevelInfoData _returnvalue_2)) (.UnlocksLevel0 (Utilities|Struct|BreakS_LevelInfoData _returnvalue_2)) (.UnlocksLevel1 (Utilities|Struct|BreakS_LevelInfoData _returnvalue_2)))))))
  (bind _outrownames_2 (DataTable|GetDataTableRowNames (Variables|Default|GetCollDataTableRef)))
  (for _array_element_2 _outrownames_2
    (bind _returnvalue_3 (Utilities|GetDataTableRow (Variables|Default|GetCollDataTableRef) _array_element_2)
      (:then
        (Utilities|Array|Add (Variables|/Game/Blueprints/SaveGame/GrimDigSaveGameObject.GrimDigSaveGameObject_C|GetCollectiblesData (Variables|Default|GetSaveGameData)) _returnvalue_3))))
  (SaveGame|SaveGametoSlot (Variables|Default|GetSaveGameData) (Variables|Default|GetSaveSlotName)))