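; BP_TextWalkIn is a walk-in trigger actor that shows on-screen text while a GrimDigPawn stands inside its box.
; On BeginPlay it creates a UI_Reading widget and fills it with TextToShow.
; Box overlap adds the widget to the viewport, and leaving removes it, destroying the actor if Destroy is set, which allows one-time messages.
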(event OnComponentBeginOverlap(Box)
  (params (OverlappedComponent :type Primitive%20Component%20Object%20Reference) (OtherActor :type Actor%20Object%20Reference) (OtherComp :type Primitive%20Component%20Object%20Reference) (OtherBodyIndex :type Integer) (bFromSweep :type Boolean) (SweepResult :type Hit%20Result%20Structure%20%28by%20ref%29))
  (Utilities|Casting|CastToGrimDigPawn OtherActor)
  (UserInterface|Viewport|AddtoViewport (Variables|Default|GetWidgetRef) 0))

(event OnComponentEndOverlap(Box)
  (params (OverlappedComponent :type Primitive%20Component%20Object%20Reference) (OtherActor :type Actor%20Object%20Reference) (OtherComp :type Primitive%20Component%20Object%20Reference) (OtherBodyIndex :type Integer))
  (Utilities|Casting|CastToGrimDigPawn OtherActor)
  (Widget|RemovefromParent (Variables|Default|GetWidgetRef))
  (if (Variables|Default|GetDestroy?)
    (Actor|DestroyActor)))

(event EventBeginPlay
  (bind _returnvalue (UserInterface|CreateWidget "/Game/Blueprints/UI/UI_Reading.UI_Reading_C"))
  (Rendering|Components|TextRender|SetText (Variables|/Game/Blueprints/UI/UI_Reading.UI_Reading_C|GetTextBlock_103 _returnvalue) (Variables|Default|GetTextToShow))
  (Variables|Default|SetWidgetRef _returnvalue))

(event Collision|EventActorBeginOverlap
  (params (OtherActor :type Actor%20Object%20Reference)))

(event EventTick
  (params (DeltaSeconds :type Float%20%28single-precision%29)))

(fn ConstructionScript)