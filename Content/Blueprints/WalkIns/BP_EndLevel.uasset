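; Level-end actor for GrimDig that tallies the gold and secrets found, then opens the end-of-level screen.
; After a short BeginPlay delay it totals all gold and secrets, while separately caching the levels this one unlocks from GameInstance save data.
; EndLevel derives found gold by subtracting what remains in the world, counts flagged secrets, then passes itself and the player to UI_EndLevel under UI-only input.
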(event Custom|EndLevel
  (params (PlayerRef :type Grim%20Dig%20Pawn%20Object%20Reference))
  (bind _returnvalue (Game|GetPlayerController 0))
  (Utilities|CountGold)
  (Utilities|CountSecrets)
  (Variables|/Game/Blueprints/Character/GrimDigPawn.GrimDigPawn_C|SetKeyPressed PlayerRef "NewEnumerator4")
  (bind _returnvalue_2 (UserInterface|CreateWidget "/Game/Blueprints/UI/UI_EndLevel.UI_EndLevel_C"))
  (UserInterface|Viewport|AddtoViewport _returnvalue_2 0)
  (Variables|/Game/Blueprints/UI/UI_EndLevel.UI_EndLevel_C|SetPlayerRef _returnvalue_2 PlayerRef)
  (Variables|/Game/Blueprints/UI/UI_EndLevel.UI_EndLevel_C|SetEndLevelObjectRef _returnvalue_2 self)
  (Variables|/Script/Engine.PlayerController|SetbShowMouseCursor _returnvalue true)
  (Input|SetInputModeUIOnly _returnvalue _returnvalue_2 "DoNotLock"))

(event EventBeginPlay
  (bind _unlocklevelnames (Variables|Default|GetUnlockLevelNames))
  (Utilities|FlowControl|Sequence
    (:then_0
      (Utilities|FlowControl|Delay 0.2)
      (bind _outactors (Actor|GetAllActorsOfClass "/Game/Blueprints/Interactibles/BP_BaseGold.BP_BaseGold_C"))
      (for _array_element _outactors
        (Variables|Default|SetTotal%20Gold%20on%20Level (+ (Variables|/Game/Blueprints/Interactibles/BP_BaseGold.BP_BaseGold_C|GetAmountOfGold _array_element) (Variables|Default|GetTotal%20Gold%20on%20Level))))
      (bind _outactors_2 (Actor|GetAllActorsOfClass "/Game/Blueprints/Interactibles/BP_GoldNugget.BP_GoldNugget_C"))
      (for _array_element_2 _outactors_2
        (Variables|Default|SetTotal%20Gold%20on%20Level (+ (Variables|/Game/Blueprints/Interactibles/BP_GoldNugget.BP_GoldNugget_C|GetAmountOfGold _array_element_2) (Variables|Default|GetTotal%20Gold%20on%20Level))))
      (Development|PrintString (Utilities|String|Append "Total Gold on Level:" (Utilities|String|ToString(Integer) (Variables|Default|GetTotal%20Gold%20on%20Level))))
      (bind _outactors_3 (Actor|GetAllActorsOfClass "/Game/Blueprints/WalkIns/BP_Secret.BP_Secret_C"))
      (for _array_element_3 _outactors_3
        (Math|Integer|IncrementInt (Variables|Default|GetSecretsOnLevel))))
    (:then_1
      (bind _returnvalue (Game|GetCurrentLevelName true))
      (Variables|Default|SetCurrentLevel (Utilities|String|StringToName _returnvalue)))
    (:then_2
      (bind _asgrim_dig_game_instance (Utilities|Casting|CastToGrimDigGameInstance (Game|GetGameInstance)))
      (Variables|Default|SetGameInstanceRef _asgrim_dig_game_instance))
    (:then_3
      (bind _levelindex (Default|FindLevelOfName (Variables|Default|GetGameInstanceRef) (Variables|Default|GetCurrentLevel)))
      (Utilities|Array|Clear _unlocklevelnames)
      (Utilities|Array|Add _unlocklevelnames (.UnlocksLevel0 (Utilities|Struct|BreakS_LevelInfoData (Utilities|Array|Get(acopy) (Variables|/Game/Blueprints/SaveGame/GrimDigSaveGameObject.GrimDigSaveGameObject_C|GetLevelData (Variables|/Game/Blueprints/SaveGame/GrimDigGameInstance.GrimDigGameInstance_C|GetSaveGameData (Variables|Default|GetGameInstanceRef))) _levelindex))))
      (Utilities|Array|Add _unlocklevelnames (.UnlocksLevel1 (Utilities|Struct|BreakS_LevelInfoData (Utilities|Array|Get(acopy) (Variables|/Game/Blueprints/SaveGame/GrimDigSaveGameObject.GrimDigSaveGameObject_C|GetLevelData (Variables|/Game/Blueprints/SaveGame/GrimDigGameInstance.GrimDigGameInstance_C|GetSaveGameData (Variables|Default|GetGameInstanceRef))) _levelindex)))))))

(event Collision|EventActorBeginOverlap
  (params (OtherActor :type Actor%20Object%20Reference)))

(event EventTick
  (params (DeltaSeconds :type Float%20%28single-precision%29)))

(fn ConstructionScript)