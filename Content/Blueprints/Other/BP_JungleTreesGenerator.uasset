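; Tree cluster generator that dresses its "Tree"-tagged components as one TreeType, from jungle, autumn and pine to snowed, burnt or stumps.
; The construction script gives each component a PickTreeType mesh plus random XY offset, yaw and non-uniform scale.
; A random stream, optionally reseeded by GenerateSeed, drives the variation; PickTreeType's per-type tables include empty slots.
; On BeginPlay, Block collision becomes query-only, or disabled for stumps.
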(event EventBeginPlay
  (Collision|SetCollisionEnabled (Variables|Default|GetBlock) (Utilities|Select :Index (Variables|Default|GetTreeType) :NewEnumerator0 "QueryOnly" :NewEnumerator1 "QueryOnly" :NewEnumerator2 "QueryOnly" :NewEnumerator3 "QueryOnly" :NewEnumerator10 "QueryOnly" :NewEnumerator4 "QueryOnly" :NewEnumerator5 "QueryOnly" :NewEnumerator6 "QueryOnly" :NewEnumerator7 "QueryOnly" :NewEnumerator8 "QueryOnly" :NewEnumerator9 "NoCollision")))

(event Collision|EventActorBeginOverlap
  (params (OtherActor :type Actor%20Object%20Reference)))

(event EventTick
  (params (DeltaSeconds :type Float%20%28single-precision%29)))

(fn ConstructionScript
  (bind _streamvar (Variables|Default|GetStreamVar))
  (bind _returnvalue (Math|Random|RandomFloatinRangefromStream 0.5 1.5 _streamvar))
  (if (Variables|Default|GetGenerateSeed?)
    (Math|Random|SetRandomStreamSeed (Variables|Default|GetStreamVar) (Math|Random|RandomInteger 99999)))
  (for _array_element (Actor|GetComponentsbyTag "/Script/Engine.SceneComponent" "Tree")
    (Components|StaticMesh|SetStaticMesh (.AsStatic%20Mesh%20Component (Utilities|Casting|CastToStaticMeshComponent _array_element)) (Utilities|PickTreeType))
    (Transformation|AddRelativeLocation _array_element (Math|Vector|MakeVector (Math|Random|RandomFloatinRangefromStream -25.0 25.0 (Variables|Default|GetStreamVar)) (Math|Random|RandomFloatinRangefromStream -25.0 25.0 (Variables|Default|GetStreamVar)) 0.0) false false)
    (Transformation|AddRelativeRotation _array_element (Math|Rotator|MakeRotator 0.0 0.0 (Math|Random|RandomFloatinRangefromStream 0.0 3.6e+02 (Variables|Default|GetStreamVar))) false false)
    (Transformation|SetRelativeScale3D _array_element (Math|Vector|MakeVector _returnvalue _returnvalue _returnvalue))))