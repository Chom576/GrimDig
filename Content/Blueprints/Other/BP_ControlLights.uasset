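; BP_ControlLights is an overlap trigger that changes the scene's lighting when the GrimDigPawn enters it, optionally switching off the pawn's torch through HasLight.
; It finds directional lights and skylights tagged "Sun" and uses two timelines to blend their intensities from current to desired values.
; Each timeline restarts inside its loop, so the setup effectively assumes one tagged light of each type.
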(event EventBeginPlay)

(event Collision|EventActorBeginOverlap
  (params (OtherActor :type Actor%20Object%20Reference))
  (bind _asgrim_dig_pawn (Utilities|Casting|CastToGrimDigPawn OtherActor))
  (if (Variables|Default|GetTurnOffTorch?)
    (Variables|/Game/Blueprints/Character/GrimDigPawn.GrimDigPawn_C|SetHasLight _asgrim_dig_pawn false))
  (bind _outactors (Actor|GetAllActorsOfClasswithTag "/Script/Engine.DirectionalLight" "Sun"))
  (for _array_element _outactors
    (Variables|Default|SetCurrentDirectionalIntensity (Variables|/Script/Engine.LightComponentBase|GetIntensity (Variables|/Script/Engine.Light|GetLightComponent _array_element)))
    (bind _newtrack_0 (Timeline|Timeline_0 PlayFromStart)
      (:Update
        (Rendering|Components|Light|SetIntensity (Variables|/Script/Engine.Light|GetLightComponent _array_element) (Math|Float|Lerp (Variables|Default|GetCurrentDirectionalIntensity) (Variables|Default|GetDesiredDirectionalIntensity) _newtrack_0)))))
  (bind _outactors_2 (Actor|GetAllActorsOfClasswithTag "/Script/Engine.SkyLight" "Sun"))
  (for _array_element_2 _outactors_2
    (Variables|Default|SetCurrentSkylightIntensity (Variables|/Script/Engine.LightComponentBase|GetIntensity (Variables|/Script/Engine.SkyLight|GetLightComponent _array_element_2)))
    (bind _newtrack_0_2 (Timeline|Timeline_1 PlayFromStart)
      (:Update
        (Rendering|Components|Light|SetIntensity (Variables|/Script/Engine.SkyLight|GetLightComponent _array_element_2) (Math|Float|Lerp (Variables|Default|GetCurrentSkylightIntensity) (Variables|Default|GetDesiredSkylightIntensity) _newtrack_0_2))))))

(event EventTick
  (params (DeltaSeconds :type Float%20%28single-precision%29)))

(fn ConstructionScript)