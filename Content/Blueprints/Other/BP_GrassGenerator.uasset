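; Grass generator actor that scatters randomized ground clutter such as plants, rocks and rubble from its construction script.
; Each component tagged "Tree" gets a random static mesh, a random horizontal offset and yaw, and a random scale per axis.
; The random index spans only 0 to 14, so most later Select options, including the moss meshes, are never picked.
; Randomization is unseeded, so each construction rerun changes the layout.
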(event EventBeginPlay)

(event Collision|EventActorBeginOverlap
  (params (OtherActor :type Actor%20Object%20Reference)))

(event EventTick
  (params (DeltaSeconds :type Float%20%28single-precision%29)))

(fn ConstructionScript
  (bind _returnvalue (Math|Random|RandomFloatinRange 0.5 1.0))
  (for _array_element (Actor|GetComponentsbyTag "/Script/Engine.SceneComponent" "Tree")
    (Components|StaticMesh|SetStaticMesh (.AsStatic%20Mesh%20Component (Utilities|Casting|CastToStaticMeshComponent _array_element)) (Utilities|Select :Index (Math|Random|RandomIntegerinRange 0 14) :Option%200 "/Game/Assets/Meshes/Plants_Small/SM_Prop_Plant_13.SM_Prop_Plant_13" :Option%201 "/Game/Assets/Meshes/Plants_Small/SM_Prop_Plant_14.SM_Prop_Plant_14" :Option%202 "/Game/Assets/Meshes/Plants_Small/SM_Prop_Plant_01.SM_Prop_Plant_01" :Option%203 "/Game/Assets/Meshes/Plants_Small/SM_Prop_Plant_02.SM_Prop_Plant_02" :Option%204 "/Game/Assets/Meshes/Plants_Small/SM_Prop_Plant_03.SM_Prop_Plant_03" :Option%205 "/Game/Assets/Meshes/Plants_Small/SM_Prop_Plant_04.SM_Prop_Plant_04" :Option%206 "/Game/Assets/Meshes/Plants_Small/SM_Prop_Plant_05.SM_Prop_Plant_05" :Option%207 "/Game/Assets/Meshes/Plants_Small/SM_Prop_Plant_11.SM_Prop_Plant_11" :Option%208 "/Game/Assets/Meshes/Plants_Small/SM_Prop_Plant_12.SM_Prop_Plant_12" :Option%209 "/Game/Assets/Meshes/RubbleAndRocks/SM_Prop_Rubble_22.SM_Prop_Rubble_22" :Option%2010 "/Game/Assets/Meshes/RubbleAndRocks/SM_Prop_Rubble_23.SM_Prop_Rubble_23" :Option%2011 "/Game/Assets/Meshes/RubbleAndRocks/SM_Prop_Rubble_24.SM_Prop_Rubble_24" :Option%2012 "/Game/Assets/Meshes/RubbleAndRocks/SM_Prop_Rocks_11.SM_Prop_Rocks_11" :Option%2013 "/Game/Assets/Meshes/RubbleAndRocks/SM_Prop_Rocks_12.SM_Prop_Rocks_12" :Option%2014 "/Game/Assets/Meshes/Plants_Small/SM_Foliage01.SM_Foliage01" :Option%2015 "/Game/Assets/Meshes/Plants_Small/SM_Foliage02.SM_Foliage02" :Option%2016 "/Game/Assets/Meshes/Plants_Small/SM_Foliage03.SM_Foliage03" :Option%2017 "/Game/Assets/Meshes/Plants_Small/SM_Foliage04.SM_Foliage04" :Option%2018 "/Game/Assets/Meshes/Plants_Small/SM_Foliage05.SM_Foliage05" :Option%2019 "/Game/Assets/Meshes/Plants_Small/SM_Foliage06.SM_Foliage06" :Option%2020 "/Game/Assets/Meshes/Plants_Small/SM_Foliage07.SM_Foliage07" :Option%2021 "/Game/Assets/Meshes/Plants_Small/SM_Foliage08.SM_Foliage08" :Option%2022 "/Game/Assets/Meshes/Plants_Small/SM_Foliage19.SM_Foliage19" :Option%2023 "/Game/Assets/Meshes/Plants_Small/SM_Foliage20.SM_Foliage20" :Option%2024 "/Game/Assets/Meshes/Plants_Small/SM_Plant01.SM_Plant01" :Option%2025 "/Game/Assets/Meshes/Plants_Small/SM_Plant02.SM_Plant02" :Option%2026 "/Game/Assets/Meshes/Plants_Small/SM_Plant03.SM_Plant03" :Option%2027 "/Game/Assets/Meshes/Plants_Small/SM_Plant04.SM_Plant04" :Option%2028 "/Game/Assets/Meshes/Plants_Small/SM_Plant05.SM_Plant05" :Option%2029 "/Game/Assets/Meshes/Plants_Small/SM_Plant06.SM_Plant06" :Option%2030 "/Game/Assets/Meshes/Plants_Small/SM_Prop_Moss_01.SM_Prop_Moss_01" :Option%2031 "/Game/Assets/Meshes/Plants_Small/SM_Prop_Moss_02.SM_Prop_Moss_02" :Option%2032 0))
    (Transformation|AddRelativeLocation _array_element (Math|Vector|MakeVector (Math|Random|RandomFloatinRange -2e+02 2e+02) (Math|Random|RandomFloatinRange -2e+02 2e+02) 0.0) false false)
    (Transformation|AddRelativeRotation _array_element (Math|Rotator|MakeRotator 0.0 0.0 (Math|Random|RandomFloatinRange 0.0 3.6e+02)) false false)
    (Transformation|SetRelativeScale3D _array_element (Math|Vector|MakeVector _returnvalue _returnvalue _returnvalue))))