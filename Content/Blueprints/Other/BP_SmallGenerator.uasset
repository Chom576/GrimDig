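; BP_SmallGenerator is a construction-script scatter actor that randomizes the layout of its components tagged "Tree".
; Each tagged component gets the chosen Mesh, a random XY offset, random yaw and independent per-axis scale between MinScale and MaxScale.
; All transform randomness draws from one random stream, which is reseeded on construction only when GenrateSeed is set.
; The event graph holds no runtime logic.
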(event EventBeginPlay)

(event Collision|EventActorBeginOverlap
  (params (OtherActor :type Actor%20Object%20Reference)))

(event EventTick
  (params (DeltaSeconds :type Float%20%28single-precision%29)))

(fn ConstructionScript
  (bind _minscale (Variables|Default|GetMinScale))
  (bind _stream (Variables|Default|GetStream))
  (bind _maxscale (Variables|Default|GetMaxScale))
  (bind _returnvalue (Math|Random|RandomFloatinRangefromStream _minscale _maxscale _stream))
  (if (Variables|Default|GetGenrateSeed?)
    (Math|Random|SetRandomStreamSeed (Variables|Default|GetStream) (Math|Random|RandomInteger 99999)))
  (for _array_element (Actor|GetComponentsbyTag "/Script/Engine.SceneComponent" "Tree")
    (Components|StaticMesh|SetStaticMesh (.AsStatic%20Mesh%20Component (Utilities|Casting|CastToStaticMeshComponent _array_element)) (Variables|Default|GetMesh))
    (Transformation|AddRelativeLocation _array_element (Math|Vector|MakeVector (Math|Random|RandomFloatinRangefromStream -2e+02 2e+02 (Variables|Default|GetStream)) (Math|Random|RandomFloatinRangefromStream -2e+02 2e+02 (Variables|Default|GetStream)) 0.0) false false)
    (Transformation|AddRelativeRotation _array_element (Math|Rotator|MakeRotator 0.0 0.0 (Math|Random|RandomFloatinRangefromStream 0.0 3.6e+02 (Variables|Default|GetStream))) false false)
    (Transformation|SetRelativeScale3D _array_element (Math|Vector|MakeVector _returnvalue _returnvalue _returnvalue))))