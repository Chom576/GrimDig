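; BP_ClimbableBricks is a climbable brick prop that varies how far each brick sits along its local X axis.
; The construction script finds static mesh components tagged "Brick" and adds a random relative X offset to each, without sweeping.
; The offsets use an unseeded random range, so the layout can change whenever construction reruns.
; The event graph holds only disabled default events, so no climbing logic runs here.
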(event EventBeginPlay
  (|CallParentFunction) ; This node is disabled and will not be called.\nDrag off pins to build functionality.
)

(event Collision|EventActorBeginOverlap
  (params (OtherActor :type Actor%20Object%20Reference))
  (|CallParentFunction OtherActor) ; This node is disabled and will not be called.\nDrag off pins to build functionality.
)

(event EventTick
  (params (DeltaSeconds :type Float%20%28single-precision%29))
  (|CallParentFunction DeltaSeconds) ; This node is disabled and will not be called.\nDrag off pins to build functionality.
)

(fn ConstructionScript
  (|CallParentFunction)
  (for _array_element (Actor|GetComponentsbyTag "/Script/Engine.StaticMeshComponent" "Brick")
    (Transformation|AddRelativeLocation _array_element (Math|Vector|MakeVector (Math|Random|RandomFloatinRange 2e+02 -1e+02) 0.0 0.0) false false)))