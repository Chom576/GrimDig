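; BP_Climbable is a climbable actor with an optional one-time scare that fakes unstable ground.
; When Scare is set, the first ScareBox overlap fires a DoOnce, continuing only for a GrimDigPawn.
; After a short delay it spawns three randomly offset dust-fall emitters above the actor and plays a world camera shake.
; The DoOnce precedes the pawn cast, so any overlapping actor uses up the scare.
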(event OnComponentBeginOverlap(ScareBox)
  (params (OverlappedComponent :type Primitive%20Component%20Object%20Reference) (OtherActor :type Actor%20Object%20Reference) (OtherComp :type Primitive%20Component%20Object%20Reference) (OtherBodyIndex :type Integer) (bFromSweep :type Boolean) (SweepResult :type Hit%20Result%20Structure%20%28by%20ref%29))
  (bind _returnvalue (Transformation|GetActorLocation))
  (bind _returnvalue_2 (Math|Random|RandomFloatinRange 2.5e+02 4.5e+02))
  (bind _returnvalue_3 (Math|Random|RandomFloatinRange -2e+02 2e+02))
  (bind _returnvalue_4 (+ _returnvalue (Math|Vector|MakeVector _returnvalue_3 0.0 _returnvalue_2)))
  (if (Variables|Default|GetScare?)
    (Utilities|FlowControl|DoOnce false
      (:Completed
        (Utilities|Casting|CastToGrimDigPawn OtherActor)
        (Utilities|FlowControl|Delay 0.2)
        (Effects|SpawnEmitteratLocation "/Game/Assets/ParticleFX/P_FX_DustFall.P_FX_DustFall" _returnvalue_4)
        (Effects|SpawnEmitteratLocation "/Game/Assets/ParticleFX/P_FX_DustFall.P_FX_DustFall" _returnvalue_4)
        (Effects|SpawnEmitteratLocation "/Game/Assets/ParticleFX/P_FX_DustFall.P_FX_DustFall" _returnvalue_4)
        (Camera|PlayWorldCameraShake "/Game/Blueprints/Interactibles/UnstableGround.UnstableGround_C" (Transformation|GetActorLocation) 0.0 5e+02)))))

(event EventBeginPlay)

(event Collision|EventActorBeginOverlap
  (params (OtherActor :type Actor%20Object%20Reference)))

(event EventTick
  (params (DeltaSeconds :type Float%20%28single-precision%29)))

(fn ConstructionScript)