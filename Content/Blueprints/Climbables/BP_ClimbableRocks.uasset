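; BP_ClimbableRocks is a climbable rock prop that builds a randomized arrangement of rock meshes in its construction script, with no active runtime logic.
; Components tagged "Brick" get random offsets, pitch and rock or stone meshes from a seeded stream.
; AddTwoOnTop reveals "Top"-tagged components with their own random offset, pitch, mesh and scale.
; GenerateSeed rerolls the stream seed whenever construction runs; otherwise the stored seed drives the layout.
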(event EventBeginPlay
  (|CallParentFunction) ; This node is disabled and will not be called.\nDrag off pins to build functionality.
)

(event Collision|EventActorBeginOverlap
  (params (OtherActor :type Actor%20Object%20Reference))
  (|CallParentFunction OtherActor) ; This node is disabled and will not be called.\nDrag off pins to build functionality.
)

(event EventTick
  (params (DeltaSeconds :type Float%20%28single-precision%29))
  (|CallParentFunction DeltaSeconds) ; This node is disabled and will not be called.\nDrag off pins to build functionality.
)

(fn ConstructionScript
  (|CallParentFunction)
  (if (Variables|Default|GetGenerateSeed)
    (Math|Random|SetRandomStreamSeed (Variables|Default|GetStreamVar) (Math|Random|RandomInteger 99999)))
  (for _array_element (Actor|GetComponentsbyTag "/Script/Engine.StaticMeshComponent" "Brick")
    (Transformation|AddRelativeLocation _array_element (Math|Vector|MakeVector (Math|Random|RandomFloatinRangefromStream -1e+02 2e+02 (Variables|Default|GetStreamVar)) 0.0 (Math|Random|RandomFloatinRangefromStream -25.0 25.0 (Variables|Default|GetStreamVar))) false false)
    (Transformation|AddRelativeRotation _array_element (Math|Rotator|MakeRotator 0.0 (Math|Random|RandomFloatinRangefromStream -9e+01 9e+01 (Variables|Default|GetStreamVar)) 0.0) false false)
    (Components|StaticMesh|SetStaticMesh _array_element (Utilities|Select :Index (Math|Random|RandomIntegerinRangefromStream 0 12 (Variables|Default|GetStreamVar)) :Option%200 "/Game/Assets/Meshes/RubbleAndRocks/SM_Rock16.SM_Rock16" :Option%201 "/Game/Assets/Meshes/RubbleAndRocks/SM_Rock17.SM_Rock17" :Option%202 "/Game/Assets/Meshes/RubbleAndRocks/SM_Rock18.SM_Rock18" :Option%203 "/Game/Assets/Meshes/RubbleAndRocks/SM_Rock19.SM_Rock19" :Option%204 "/Game/Assets/Meshes/RubbleAndRocks/SM_Rock20.SM_Rock20" :Option%205 "/Game/Assets/Meshes/RubbleAndRocks/SM_Stone02.SM_Stone02" :Option%206 "/Game/Assets/Meshes/RubbleAndRocks/SM_Stone03.SM_Stone03" :Option%207 "/Game/Assets/Meshes/RubbleAndRocks/SM_Stone05.SM_Stone05" :Option%208 "/Game/Assets/Meshes/RubbleAndRocks/SM_Stone04.SM_Stone04" :Option%209 "/Game/Assets/Meshes/RubbleAndRocks/SM_Stone01.SM_Stone01" :Option%2010 "/Game/Assets/Meshes/RubbleAndRocks/SM_Stone06.SM_Stone06" :Option%2011 "/Game/Assets/Meshes/RubbleAndRocks/SM_Stone07.SM_Stone07" :Option%2012 "/Game/Assets/Meshes/RubbleAndRocks/SM_Stone08.SM_Stone08" :Option%2013 0)))
  (if (Variables|Default|GetAddTwo%20on%20top?)
    (for _array_element_2 (Actor|GetComponentsbyTag "/Script/Engine.StaticMeshComponent" "Top")
      (Rendering|SetVisibility _array_element_2 true false)
      (Transformation|AddRelativeRotation _array_element_2 (Math|Rotator|MakeRotator 0.0 (Math|Random|RandomFloatinRangefromStream -9e+01 9e+01 (Variables|Default|GetStreamVar)) 0.0) false false)
      (Transformation|AddRelativeLocation _array_element_2 (Math|Vector|MakeVector (Math|Random|RandomFloatinRangefromStream -5e+01 5e+01 (Variables|Default|GetStreamVar)) 0.0 0.0) false false)
      (Components|StaticMesh|SetStaticMesh _array_element_2 (Utilities|Select :Index (Math|Random|RandomIntegerinRangefromStream 0 2 (Variables|Default|GetStreamVar)) :Option%200 "/Game/Assets/Meshes/RubbleAndRocks/SM_Rock16.SM_Rock16" :Option%201 "/Game/Assets/Meshes/RubbleAndRocks/SM_Rock17.SM_Rock17" :Option%202 "/Game/Assets/Meshes/RubbleAndRocks/SM_Rock20.SM_Rock20"))
      (Transformation|SetRelativeScale3D _array_element_2 (Math|Conversions|ToVector(Float) (Math|Random|RandomFloatinRangefromStream 0.8 1.2 (Variables|Default|GetStreamVar)))))))