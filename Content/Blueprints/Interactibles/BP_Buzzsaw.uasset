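; Buzzsaw trap that can start on or be switched via Activate and open/close events.
; When turned on, a looping timer flip-flops a timeline forward and backward, sliding the saw between start and end markers.
; A second timeline animates its rotation, toggled only on each turn-on.
; GrimDigPawn entering the box while it runs takes damage, repeated by a re-armed timer while still overlapping.
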(event OnComponentBeginOverlap(Box)
  (params (OverlappedComponent :type Primitive%20Component%20Object%20Reference) (OtherActor :type Actor%20Object%20Reference) (OtherComp :type Primitive%20Component%20Object%20Reference) (OtherBodyIndex :type Integer) (bFromSweep :type Boolean) (SweepResult :type Hit%20Result%20Structure%20%28by%20ref%29))
  (bind _asgrim_dig_pawn (Utilities|Casting|CastToGrimDigPawn OtherActor))
  (Variables|Default|SetPlayerRef _asgrim_dig_pawn)
  (Variables|Default|SetPlayerOverlap? true)
  (if (Variables|Default|GetIsOn)
    (Game|Damage|ApplyDamage (Variables|Default|GetPlayerRef) 1.0 0 0)
    (Utilities|Time|SetTimerbyEvent (delegate Custom|ConstanDamage) 1.0)))

(event OnComponentEndOverlap(Box)
  (params (OverlappedComponent :type Primitive%20Component%20Object%20Reference) (OtherActor :type Actor%20Object%20Reference) (OtherComp :type Primitive%20Component%20Object%20Reference) (OtherBodyIndex :type Integer))
  (Utilities|Casting|CastToGrimDigPawn OtherActor)
  (Variables|Default|SetPlayerOverlap? false))

(event Custom|SwitchSideSaw
  (if (Variables|Default|GetIsOn)
    (Utilities|FlowControl|FlipFlop
      (:A
        (bind _newtrack_0 (Timeline|Timeline_0 PlayFromStart)
          (:Update
            (Transformation|SetRelativeLocation (Variables|Default|GetBuzzSaw) (Math|Vector|Lerp(Vector) (Variables|/Script/Engine.SceneComponent|GetRelativeLocation (Variables|Default|GetSawStart)) (Variables|/Script/Engine.SceneComponent|GetRelativeLocation (Variables|Default|GetSawEnd)) _newtrack_0) false false))))
      (:B
        (Timeline|Timeline_0 ReverseFromEnd)))))

(event Custom|RunStopSaw
  (Utilities|FlowControl|FlipFlop
    (:A
      (bind _newtrack_0 (Timeline|Timeline_1 Play)
        (:Update
          (Transformation|SetRelativeRotation (Variables|Default|GetBuzzSaw) (Math|Rotator|Lerp(Rotator) "0, 0, 0" "90.000000, 0, 0" _newtrack_0 true) false false))))
    (:B
      (Timeline|Timeline_1 Stop))))

(event Custom|ConstanDamage
  (if (and (Variables|Default|GetPlayerOverlap?) (Variables|Default|GetIsOn))
    (Game|Damage|ApplyDamage (Variables|Default|GetPlayerRef) 1.0 0 0)
    (Utilities|Time|SetTimerbyEvent (delegate Custom|ConstanDamage) 1.0)))

(event EventBeginPlay
  (|CallParentFunction)
  (if (Variables|Default|GetStartOn?)
    (Variables|Default|SetIsOn true)
    (CallFunction|RunStopSaw)
    (bind _returnvalue (Utilities|Time|SetTimerbyEvent (delegate Custom|SwitchSideSaw) (Variables|Default|GetTimeToSwitch) true (Variables|Default|GetDelay?)))))

(event Collision|EventActorBeginOverlap
  (params (OtherActor :type Actor%20Object%20Reference))
  (|CallParentFunction OtherActor) ; This node is disabled and will not be called.\nDrag off pins to build functionality.
)

(event EventTick
  (params (DeltaSeconds :type Float%20%28single-precision%29))
  (|CallParentFunction DeltaSeconds))

(event EventActivate
  (params (Initiator :type Actor%20Object%20Reference))
  (if (Variables|Default|GetIsOn)
    (Utilities|Time|ClearandInvalidateTimerbyHandle (stale _returnvalue))
    (Variables|Default|SetIsOn false)
    (else
      (Variables|Default|SetIsOn true)
      (CallFunction|RunStopSaw)
      (bind _returnvalue (Utilities|Time|SetTimerbyEvent (delegate Custom|SwitchSideSaw) (Variables|Default|GetTimeToSwitch) true (Variables|Default|GetDelay?))))))

(event EventTurnOff/Close
  (params (Initiator :type Actor%20Object%20Reference))
  (Utilities|Time|ClearandInvalidateTimerbyHandle (stale EventBeginPlay _returnvalue))
  (Variables|Default|SetIsOn false))

(event EventTurnOn/Open
  (params (Initiator :type Actor%20Object%20Reference))
  (Variables|Default|SetIsOn true)
  (CallFunction|RunStopSaw)
  (bind _returnvalue (Utilities|Time|SetTimerbyEvent (delegate Custom|SwitchSideSaw) (Variables|Default|GetTimeToSwitch) true (Variables|Default|GetDelay?))))

(fn ConstructionScript
  (|CallParentFunction))