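; Interactive weight-sensitive container that reacts to the items placed in or taken from it, including a golden idol.
; On each Item event it sums the contents' weights, turning off/closing a linked activable when within the min-max range.
; Otherwise it turns on/opens that activable and toggles the player's inventory.
; It also shows a mesh while the idol is inside and triggers a second activable whenever the idol is absent.
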(event EventBeginPlay
  (|CallParentFunction) ; This node is disabled and will not be called.\nDrag off pins to build functionality.
)

(event Collision|EventActorBeginOverlap
  (params (OtherActor :type Actor%20Object%20Reference))
  (|CallParentFunction OtherActor) ; This node is disabled and will not be called.\nDrag off pins to build functionality.
)

(event EventTick
  (params (DeltaSeconds :type Float%20%28single-precision%29))
  (|CallParentFunction DeltaSeconds) ; This node is disabled and will not be called.\nDrag off pins to build functionality.
)

(event EventItem
  (params (Slot :type Integer) (ItemInfo :type S%20Item%20Info%20Structure))
  (bind _activableref (Variables|Default|GetActivableRef))
  (|CallParentFunction Slot ItemInfo)
  (Variables|Default|SetSumWeigth 0)
  (Variables|Default|SetIdolPresent false)
  (bind _array_element (Utilities|Array|ForEachLoopwithBreak (Variables|Default|GetContains))
    (:LoopBody
      (Variables|Default|SetSumWeigth (+ (.Weight (Utilities|Struct|BreakS_ItemInfo _array_element)) (Variables|Default|GetSumWeigth)))
      (if (== (.ItemClass (Utilities|Struct|BreakS_ItemInfo _array_element)) "/Game/Blueprints/Interactibles/Items/BP_GoldenIdol.BP_GoldenIdol_C")
        (Variables|Default|SetIdolPresent true)))
    (:Completed
      (if (Math|Integer|InRange(Integer) (Variables|Default|GetSumWeigth) (Variables|Default|GetMinWeigth) (Variables|Default|GetMaxWeigth))
        (Default|TurnOff/Close _activableref)
        (else
          (Default|TurnOn/Open _activableref)
          (Default|Open/CloseInventory (Variables|Default|GetPlayerRef))))
      (Rendering|SetVisibility (Variables|Default|GetStaticMesh1) (Variables|Default|GetIdolPresent) false)
      (if (not (Variables|Default|GetIdolPresent))
        (Default|Activate (Variables|Default|GetIdolTakenActivableRef))))))

(event EventInteraction
  (params (PlayerRef :type Grim%20Dig%20Pawn%20Object%20Reference))
  (|CallParentFunction PlayerRef))

(fn ConstructionScript
  (|CallParentFunction))