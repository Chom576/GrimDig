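; Interactable level collectible, one of three per-level slots picked by CollectibleIndex, backed by GrimDig save data.
; After a short delay on BeginPlay, it finds the current level's entry, then destroys itself if already found or applies the saved mesh.
; Its one-shot interaction marks it found, increments its type's count, saves, spawns a far-off camera and rotating copy, and opens a UI-only popup showing name and progress.
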(event EventBeginPlay
  (|CallParentFunction)
  (Utilities|FlowControl|Delay 0.2)
  (Utilities|FlowControl|Sequence
    (:then_0
      (bind _asgrim_dig_game_instance (Utilities|Casting|CastToGrimDigGameInstance (Game|GetGameInstance)))
      (Variables|Default|SetSaveGameRef (Variables|/Game/Blueprints/SaveGame/GrimDigGameInstance.GrimDigGameInstance_C|GetSaveGameData _asgrim_dig_game_instance)))
    (:then_1
      (bind _returnvalue (Game|GetCurrentLevelName true))
      (Variables|Default|SetCurrentLevel (Utilities|String|StringToName _returnvalue)))
    (:then_2
      (bind (_array_element _array_index) (Utilities|Array|ForEachLoopwithBreak (Variables|/Game/Blueprints/SaveGame/GrimDigSaveGameObject.GrimDigSaveGameObject_C|GetLevelData (Variables|Default|GetSaveGameRef)) :!label _label)
        (:LoopBody
          (if (Utilities|Name|Equal(Name) (.LevelName (Utilities|Struct|BreakS_LevelInfoData _array_element)) (Variables|Default|GetCurrentLevel))
            (Variables|Default|SetLevelIndexFound _array_index)
            (goto _label Break)))))
    (:then_3
      (Variables|Default|SetCollectible (Utilities|GetSaveDataCollectibleInfo)))
    (:then_4
      (if (.alreadyfound (Variables|Default|GetCollectible))
        (Actor|DestroyActor)
        (else
          (Components|StaticMesh|SetStaticMesh (Variables|Default|GetStaticMesh) (.mesh (Variables|Default|GetCollectible))))))))

(event Collision|EventActorBeginOverlap
  (params (OtherActor :type Actor%20Object%20Reference))
  (|CallParentFunction OtherActor) ; This node is disabled and will not be called.\nDrag off pins to build functionality.
)

(event EventTick
  (params (DeltaSeconds :type Float%20%28single-precision%29))
  (|CallParentFunction DeltaSeconds) ; This node is disabled and will not be called.\nDrag off pins to build functionality.
)

(event EventInteraction
  (params (PlayerRef :type Grim%20Dig%20Pawn%20Object%20Reference))
  (bind _returnvalue (Game|GetPlayerController 0))
  (Utilities|FlowControl|DoOnce false
    (:Completed
      (Utilities|SetSaveDataCollectibleInfo)
      (Utilities|AddtoCollection
        (:Completed
          (Default|SaveLevelData (.AsGrim%20Dig%20Game%20Instance (Utilities|Casting|CastToGrimDigGameInstance (Game|GetGameInstance))))
          (bind _returnvalue_2 (Game|SpawnActorfromClass "/Game/Blueprints/Interactibles/BP_CollectibleCamera.BP_CollectibleCamera_C" (Math|Transform|MakeTransform (Math|Vector|MakeVector 5.783e+06 5.783e+06 0.0) "0, 0, 0" "1,1,1") "Undefined" 0 0))
          (Variables|Default|SetCaptureCameraRef _returnvalue_2)
          (bind _returnvalue_3 (Game|SpawnActorfromClass "/Game/Blueprints/Interactibles/BP_CollectibleRotating.BP_CollectibleRotating_C" (Math|Transform|MakeTransform (Math|Vector|MakeVector 5.783e+06 5.783e+06 0.0) "0, 0, 0" "1,1,1") "Undefined" 0 0))
          (bind _output_get (Variables|Default|SetRotatingCollectibleRef _returnvalue_3))
          (Components|StaticMesh|SetStaticMesh (Variables|/Game/Blueprints/Interactibles/BP_CollectibleRotating.BP_CollectibleRotating_C|GetStaticMesh _output_get) (Variables|/Script/Engine.StaticMeshComponent|GetStaticMesh (Variables|Default|GetStaticMesh)))
          (bind _returnvalue_4 (UserInterface|CreateWidget "/Game/Blueprints/UI/UI_Collectible.UI_Collectible_C"))
          (Variables|/Game/Blueprints/UI/UI_Collectible.UI_Collectible_C|SetActorRef _returnvalue_4 self)
          (Rendering|Components|TextRender|SetText (Variables|/Game/Blueprints/UI/UI_Collectible.UI_Collectible_C|GetTextBlock_143 _returnvalue_4) (Utilities|Text|ToText(String) (Utilities|String|Append "You found the " (.name (Variables|Default|GetCollectible)) "!")))
          (Rendering|Components|TextRender|SetText (Variables|/Game/Blueprints/UI/UI_Collectible.UI_Collectible_C|GetCollectibleCount _returnvalue_4) (Utilities|Text|ToText(String) (Utilities|String|Append (Utilities|String|ToString(Integer) (Variables|Default|GetNewFoundColl)) " of " (Utilities|String|ToString(Integer) (Variables|Default|GetAllCollOfType)))))
          (UserInterface|Viewport|AddtoViewport _returnvalue_4 0)
          (Input|SetInputModeUIOnly _returnvalue _returnvalue_4 "DoNotLock")
          (Variables|/Script/Engine.PlayerController|SetbShowMouseCursor _returnvalue true))))))

(fn ConstructionScript
  (|CallParentFunction))