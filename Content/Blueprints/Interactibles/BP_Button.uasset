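; BP_Button is an interactible button that triggers other objects in the level when its Interaction event fires.
; Interaction walks three lists, TurnOnList, TurnOffList and ActivateList, calling TurnOnOpen, TurnOffClose or Activate on each valid entry.
; The button holds no state or visual feedback in its graphs, and BeginPlay, overlap and Tick are unused.
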(event EventBeginPlay
  (|CallParentFunction) ; This node is disabled and will not be called.\nDrag off pins to build functionality.
)

(event Collision|EventActorBeginOverlap
  (params (OtherActor :type Actor%20Object%20Reference))
  (|CallParentFunction OtherActor) ; This node is disabled and will not be called.\nDrag off pins to build functionality.
)

(event EventTick
  (params (DeltaSeconds :type Float%20%28single-precision%29))
  (|CallParentFunction DeltaSeconds) ; This node is disabled and will not be called.\nDrag off pins to build functionality.
)

(event EventInteraction
  (params (PlayerRef :type Grim%20Dig%20Pawn%20Object%20Reference))
  (bind _turnonlist (Variables|Default|GetTurnOnList))
  (bind _turnofflist (Variables|Default|GetTurnOffList))
  (bind _activatelist (Variables|Default|GetActivateList))
  (if (> (Utilities|Array|Length _turnonlist) 0)
    (for _array_element _turnonlist
      (Utilities|IsValid _array_element
        (:Is%20Valid
          (Default|TurnOn/Open _array_element)))))
  (if (> (Utilities|Array|Length _turnofflist) 0)
    (for _array_element_2 _turnofflist
      (Utilities|IsValid _array_element_2
        (:Is%20Valid
          (Default|TurnOff/Close _array_element_2)))))
  (if (> (Utilities|Array|Length _activatelist) 0)
    (for _array_element_3 _activatelist
      (Utilities|IsValid _array_element_3
        (:Is%20Valid
          (Default|Activate _array_element_3))))))

(fn ConstructionScript
  (|CallParentFunction))