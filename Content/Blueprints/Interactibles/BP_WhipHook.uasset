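; Whip hook interactible that swings the player between predefined pairs of anchor points, mapped both ways on BeginPlay.
; WhipInteract matches the player's location to a point, takes its partner and validates the path with the player's trace functions.
; Any wall or floor hit blocks the swing, with extra samples for long jumps.
; Safe swings show the cable and move the player by timeline lerp plus Z offset; otherwise a comment prompt appears.
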(event Collision|EventActorBeginOverlap
  (params (OtherActor :type Actor%20Object%20Reference))
  (|CallParentFunction OtherActor) ; This node is disabled and will not be called.\nDrag off pins to build functionality.
)

(event EventTick
  (params (DeltaSeconds :type Float%20%28single-precision%29))
  (|CallParentFunction DeltaSeconds) ; This node is disabled and will not be called.\nDrag off pins to build functionality.
)

(event EventWhipInteract
  (params (PlayerRef :type Grim%20Dig%20Pawn%20Object%20Reference))
  (Variables|Default|SetPlayerRef PlayerRef)
  (Variables|Default|SetPlayerStart (Transformation|GetActorLocation PlayerRef))
  (Variables|Default|SetFoundPoint false)
  (bind _array_element (Utilities|Array|ForEachLoopwithBreak (Variables|Default|GetPointList) :!label _label)
    (:LoopBody
      (if (Math|Vector|Equal(Vector) (Variables|Default|GetPlayerStart) (Transformation|GetWorldLocation _array_element) 5e+01)
        (if (.ReturnValue (Utilities|Map|Find (Variables|Default|GetPoints) _array_element))
          (Variables|Default|SetFoundPoint true)
          (Variables|Default|SetProperEndPoint (.Value (Utilities|Map|Find (Variables|Default|GetPoints) _array_element)))
          (goto _label Break))))
    (:Completed
      (if (Variables|Default|GetFoundPoint)
        (Variables|Default|SetPlayerEnd (Transformation|GetWorldLocation (Variables|Default|GetProperEndPoint)))
        (bind _canjump (Utilities|TraceforSafeSwing)
          (:Out
            (if _canjump
              (Default|HideGrid (Variables|Default|GetPlayerRef))
              (Default|WhipCableShowUp (Variables|Default|GetPlayerRef))
              (Utilities|FlowControl|Delay 0.5)
              (Variables|/Game/Blueprints/Character/GrimDigPawn.GrimDigPawn_C|SetMovementInProgress (Variables|Default|GetPlayerRef) true)
              (bind (_direction _pawnmovementtimeline _zaxis) (Timeline|Timeline_0 PlayFromStart)
                (:Update
                  (Transformation|SetActorLocation (Variables|Default|GetPlayerRef) (+ (Math|Vector|Lerp(Vector) (Variables|Default|GetPlayerStart) (Variables|Default|GetPlayerEnd) _pawnmovementtimeline) (Math|Vector|MakeVector 0.0 0.0 _zaxis)) false false))
                (:Finished
                  (Default|EndMovement (Variables|Default|GetPlayerRef))
                  (Default|WhipCableHide (Variables|Default|GetPlayerRef))))
              (else
                (Default|PromptComment (Variables|Default|GetPlayerRef) "Not a safe jump." :!label _label_2)))))
        (else
          (goto _label_2))))))

(event EventBeginPlay
  (Utilities|DefinePoints))

(fn ConstructionScript
  (|CallParentFunction))