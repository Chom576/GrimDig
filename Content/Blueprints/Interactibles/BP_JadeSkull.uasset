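; Interactible physics jade skull that the player can retrieve as a weapon.
; On interaction, if that weapon slot is unlocked, it destroys itself when the player already holds a skull, otherwise it has the player equip the weapon and call RetrieveSkull.
; On mesh hits, it bounces by redirecting its current speed along the hit normal, halving the vertical component.
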(event OnComponentHit(StaticMesh)
  (params (HitComponent :type Primitive%20Component%20Object%20Reference) (OtherActor :type Actor%20Object%20Reference) (OtherComp :type Primitive%20Component%20Object%20Reference) (NormalImpulse :type Vector :default "0, 0, 0") (Hit :type Hit%20Result%20Structure%20%28by%20ref%29))
  (bind _staticmesh (Variables|Default|GetStaticMesh))
  (bind _returnvalue (Physics|GetPhysicsLinearVelocity _staticmesh "None"))
  (Physics|SetPhysicsLinearVelocity _staticmesh (Math|Vector|MakeVector (/ (.X (Math|Vector|BreakVector (* (.Normal (Collision|BreakHitResult Hit)) (Math|Vector|VectorLength _returnvalue)))) 1.0) (/ (.Y (Math|Vector|BreakVector (* (.Normal (Collision|BreakHitResult Hit)) (Math|Vector|VectorLength _returnvalue)))) 1.0) (/ (.Z (Math|Vector|BreakVector (* (.Normal (Collision|BreakHitResult Hit)) (Math|Vector|VectorLength _returnvalue)))) 2.0)) false "None"))

(event EventBeginPlay
  (|CallParentFunction) ; This node is disabled and will not be called.\nDrag off pins to build functionality.
)

(event Collision|EventActorBeginOverlap
  (params (OtherActor :type Actor%20Object%20Reference))
  (|CallParentFunction OtherActor) ; This node is disabled and will not be called.\nDrag off pins to build functionality.
)

(event EventTick
  (params (DeltaSeconds :type Float%20%28single-precision%29))
  (|CallParentFunction DeltaSeconds) ; This node is disabled and will not be called.\nDrag off pins to build functionality.
)

(event EventInteraction
  (params (PlayerRef :type Grim%20Dig%20Pawn%20Object%20Reference))
  (bind _output_get (Default|FindWeaponIndex PlayerRef "NewEnumerator3"))
  (if (.unlocked? (Utilities|Array|Get(acopy) (Variables|/Game/Blueprints/Character/GrimDigPawn.GrimDigPawn_C|GetWeaponList PlayerRef) _output_get))
    (if (Variables|/Game/Blueprints/Character/GrimDigPawn.GrimDigPawn_C|GetSkullInHand? PlayerRef)
      (Actor|DestroyActor)
      (else
        (Default|EquipWeapon PlayerRef "NewEnumerator3")
        (Default|RetrieveSkull PlayerRef)))))

(fn ConstructionScript
  (|CallParentFunction))