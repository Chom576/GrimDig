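; BR_ReadMe is a readable interactable that toggles a reading widget showing its text when the player interacts with it.
; The widget is created and filled at BeginPlay, and opening it plays a paper sound attached to the player.
; While it is open, a looping timer closes it once the player moves too far away.
; On the first read only, it can also teach the player some of a language.
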(event Custom|RemoveWidgetIfPLayerIsFar
  (if (and (> (Transformation|GetDistanceTo (stale EventInteraction PlayerRef) self) 5e+02) (UserInterface|Viewport|IsinViewport (Variables|Default|GetWidgetRef)))
    (Widget|RemovefromParent (Variables|Default|GetWidgetRef))
    (Utilities|Time|ClearandInvalidateTimerbyHandle (stale EventInteraction _returnvalue))))

(event EventBeginPlay
  (|CallParentFunction)
  (bind _returnvalue (UserInterface|CreateWidget "/Game/Blueprints/UI/UI_Reading.UI_Reading_C"))
  (Rendering|Components|TextRender|SetText (Variables|/Game/Blueprints/UI/UI_Reading.UI_Reading_C|GetTextBlock_103 _returnvalue) (Variables|Default|GetTextToRead))
  (Variables|Default|SetWidgetRef _returnvalue))

(event Collision|EventActorBeginOverlap
  (params (OtherActor :type Actor%20Object%20Reference))
  (|CallParentFunction OtherActor) ; This node is disabled and will not be called.\nDrag off pins to build functionality.
)

(event EventTick
  (params (DeltaSeconds :type Float%20%28single-precision%29))
  (|CallParentFunction DeltaSeconds) ; This node is disabled and will not be called.\nDrag off pins to build functionality.
)

(event EventInteraction
  (params (PlayerRef :type Grim%20Dig%20Pawn%20Object%20Reference))
  (bind _widgetref (Variables|Default|GetWidgetRef))
  (if (UserInterface|Viewport|IsinViewport _widgetref)
    (Widget|RemovefromParent _widgetref)
    (Utilities|Time|ClearandInvalidateTimerbyHandle (stale _returnvalue))
    (else
      (UserInterface|Viewport|AddtoViewport _widgetref 0)
      (Audio|SpawnSoundAttached "/Game/Assets/Audio/SFX_OGG/RandomPaper_Cue.RandomPaper_Cue" (Variables|/Game/Blueprints/Character/GrimDigPawn.GrimDigPawn_C|GetScene PlayerRef) "None" "0, 0, 0" "0, 0, 0" "KeepRelativeOffset" false 1.0 1.0 0.0 0 0)
      (bind _returnvalue (Utilities|Time|SetTimerbyEvent (delegate Custom|RemoveWidgetIfPLayerIsFar) 1.0 true))
      (Utilities|FlowControl|DoOnce false
        (:Completed
          (if (Variables|Default|GetLearnLanguage)
            (Default|LearnLanguage PlayerRef (Variables|Default|GetWhatLanguage?) (Variables|Default|GetLanguageAmount))))))))

(fn ConstructionScript
  (|CallParentFunction))