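; BP_LightSource is an interactable fire light source that passes flame to and from the player's torch.
; A plain interaction prompts the player to equip a torch.
; A torch interaction gives light to an unlit player if the source is alight, or lights the source if the player carries light.
; IsAlight drives particle and point light visibility, applied in the construction script for pre-lit instances.
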(event EventBeginPlay
  (|CallParentFunction))

(event Collision|EventActorBeginOverlap
  (params (OtherActor :type Actor%20Object%20Reference))
  (|CallParentFunction OtherActor) ; This node is disabled and will not be called.\nDrag off pins to build functionality.
)

(event EventTick
  (params (DeltaSeconds :type Float%20%28single-precision%29))
  (|CallParentFunction DeltaSeconds) ; This node is disabled and will not be called.\nDrag off pins to build functionality.
)

(event EventInteraction
  (params (PlayerRef :type Grim%20Dig%20Pawn%20Object%20Reference))
  (Default|PromptComment PlayerRef "I should equip a torch."))

(event EventTorchInteract
  (params (PlayerRef :type Grim%20Dig%20Pawn%20Object%20Reference))
  (bind _haslight (Variables|/Game/Blueprints/Character/GrimDigPawn.GrimDigPawn_C|GetHasLight PlayerRef))
  (if (Variables|Default|GetIsAlight?)
    (if (not _haslight)
      (Default|GainTorch PlayerRef))
    (elif _haslight
      (Variables|Default|SetIsAlight? true)
      (Rendering|SetVisibility (Variables|Default|GetParticleSystem) true false))))

(fn ConstructionScript
  (|CallParentFunction)
  (if (Variables|Default|GetIsAlight?)
    (Rendering|SetVisibility (Variables|Default|GetParticleSystem) true false)))