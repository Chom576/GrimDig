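; Interactable box that the player grabs from alongside and pushes or pulls one step at a time.
; Push and pull are refused with a wall bump when another box sits on top or traces detect obstructions, or missing floor behind a pulling player.
; Valid moves lerp player and box together on timelines with scrape sounds.
; Without ground afterwards, the box releases the player and drops in fixed steps until it lands with a thump.
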(event Custom|PushBox
  (bind _returnvalue (Transformation|GetActorLocation))
  (bind _playerref (Variables|Default|GetPlayerRef))
  (bind _playerref_2 (Variables|Default|GetPlayerRef))
  (bind _is_there_box_on_top_ (CallFunction|LookforBoxonTop))
  (if _is_there_box_on_top_
    (Default|SetStartandEndPointforMovementFunction _playerref 1 "NewEnumerator0")
    (Default|WallBump _playerref true)
    (else
      (Utilities|SetPushCoordinates)
      (bind _foundwall (Default|TraceforWall (Variables|Default|GetPlayerRef) (Variables|Default|GetBoxStart) (Variables|Default|GetBoxEnd) true self))
      (if _foundwall
        (Default|SetStartandEndPointforMovementFunction _playerref_2 1 "NewEnumerator0")
        (Default|WallBump _playerref_2 true)
        (else
          (Audio|PlaySoundatLocation "/Game/Assets/Audio/SFX_OGG/damaged1_Cue.damaged1_Cue" _returnvalue "0, 0, 0" 1.0 1.0 0.0 "/Game/Assets/Audio/NewSoundAttenuation.NewSoundAttenuation" 0 0)
          (Audio|PlaySoundatLocation "/Game/Assets/Audio/SFX_OGG/SFX_-_stone_scrape_02.SFX_-_stone_scrape_02" _returnvalue "0, 0, 0" 1.0 1.0 0.0 "/Game/Assets/Audio/NewSoundAttenuation.NewSoundAttenuation" 0 0)
          (bind (_direction _playermovementtimeline _boxmovementtimeline) (Timeline|Timeline_0 PlayFromStart)
            (:Update
              (Transformation|SetActorLocation (Variables|Default|GetPlayerRef) (Math|Vector|Lerp(Vector) (Variables|Default|GetPlayerStart) (Variables|Default|GetBoxStart) _playermovementtimeline) false false)
              (Transformation|SetActorLocation (Math|Vector|Lerp(Vector) (Variables|Default|GetBoxStart) (Variables|Default|GetBoxEnd) _boxmovementtimeline) false false))
            (:Finished
              (CallFunction|EndPushPullMovement))))))))

(event Custom|PullBox
  (bind _returnvalue (Transformation|GetActorLocation))
  (bind _playerref (Variables|Default|GetPlayerRef))
  (bind _playerref_2 (Variables|Default|GetPlayerRef))
  (bind _playerref_3 (Variables|Default|GetPlayerRef))
  (bind _playerref_4 (Variables|Default|GetPlayerRef))
  (bind _is_there_box_on_top_ (CallFunction|LookforBoxonTop))
  (if _is_there_box_on_top_
    (Default|SetStartandEndPointforMovementFunction _playerref_2 1 "NewEnumerator3")
    (Default|WallBump _playerref_2 false)
    (else
      (Utilities|SetPullCoordinates)
      (bind _foundwall (Default|TraceforWall (Variables|Default|GetPlayerRef) (Variables|Default|GetPlayerStart) (Variables|Default|GetPlayerEnd) false))
      (if _foundwall
        (Default|SetStartandEndPointforMovementFunction _playerref_4 1 "NewEnumerator3" :!label _label)
        (Default|WallBump _playerref_4 true)
        (else
          (bind _foundwall_2 (Default|TraceforWall _playerref_3 (Variables|Default|GetPlayerStart) (Variables|Default|GetPlayerEnd) true))
          (if _foundwall_2
            (bind _foundfloor (Default|TraceforFloor _playerref_3 (+ (Variables|Default|GetPlayerEnd) "0, 0,250.000000")))
            (if _foundfloor
              (goto _label)
              (else
                _)))
          (bind _foundwall_3 (Default|TraceforWall _playerref_3 (Variables|Default|GetBoxStart) (Variables|Default|GetPlayerStart) true self))
          (if _foundwall_3
            (goto _label)
            (else
              (bind _foundfloor_2 (Default|TraceforFloor _playerref_3 (Variables|Default|GetPlayerEnd)))
              (if _foundfloor_2
                (Audio|PlaySoundatLocation "/Game/Assets/Audio/SFX_OGG/damaged1_Cue.damaged1_Cue" _returnvalue "0, 0, 0" 1.0 1.0 0.0 "/Game/Assets/Audio/NewSoundAttenuation.NewSoundAttenuation" 0 0)
                (Audio|PlaySoundatLocation "/Game/Assets/Audio/SFX_OGG/SFX_-_stone_scrape_02.SFX_-_stone_scrape_02" _returnvalue "0, 0, 0" 1.0 1.0 0.0 "/Game/Assets/Audio/NewSoundAttenuation.NewSoundAttenuation" 0 0)
                (bind (_direction _pawnmovementtimeline _boxmovementtimeline) (Timeline|Timeline_1 PlayFromStart)
                  (:Update
                    (Transformation|SetActorLocation (Variables|Default|GetPlayerRef) (Math|Vector|Lerp(Vector) (Variables|Default|GetPlayerStart) (Variables|Default|GetPlayerEnd) _pawnmovementtimeline) false false)
                    (Transformation|SetActorLocation (Math|Vector|Lerp(Vector) (Variables|Default|GetBoxStart) (Variables|Default|GetPlayerStart) _boxmovementtimeline) false false))
                  (:Finished
                    (CallFunction|EndPushPullMovement)))
                (else
                  (Default|SetStartandEndPointforMovementFunction _playerref 1 "NewEnumerator3")
                  (Default|WallBump _playerref false))))))))))

(event Custom|EndPushPullMovement
  (bind _returnvalue (Transformation|GetActorLocation))
  (bind _returnvalue_2 (Collision|LineTraceByChannel (+ _returnvalue "0, 0,300.000000") (+ _returnvalue "0, 0,-200.000000") "TraceTypeQuery1" false 0 "None"))
  (if _returnvalue_2
    (if (Variables|Default|GetWasFalling)
      (Audio|PlaySoundatLocation "/Game/Assets/Audio/SFX_OGG/SFX_-_thump_01.SFX_-_thump_01" (Transformation|GetActorLocation) "0, 0, 0" 1.0 1.0 0.0 "/Game/Assets/Audio/NewSoundAttenuation.NewSoundAttenuation" 0 0)
      (Variables|Default|SetWasFalling false))
    (Default|EndMovement (Variables|Default|GetPlayerRef))
    (else
      (CallFunction|BreakPushPull)
      (CallFunction|ShortLanding))))

(event Custom|ShortLanding
  (bind _returnvalue (Transformation|GetActorLocation))
  (Variables|Default|SetBoxStart _returnvalue)
  (Variables|Default|SetBoxEnd (+ _returnvalue "0, 0,-250.000000"))
  (bind _newtrack_0 (Timeline|Timeline_3 PlayFromStart)
    (:Update
      (Transformation|SetActorLocation (Math|Vector|Lerp(Vector) (Variables|Default|GetBoxStart) (Variables|Default|GetBoxEnd) _newtrack_0) false false))
    (:Finished
      (Variables|Default|SetWasFalling true)
      (CallFunction|EndPushPullMovement))))

(event Custom|BreakPushPull
  (bind _playerref (Variables|Default|GetPlayerRef))
  (Utilities|IsValid (Variables|Default|GetPlayerRef)
    (:Is%20Valid
      (Variables|/Game/Blueprints/Character/GrimDigPawn.GrimDigPawn_C|SetPushPullBoxRef _playerref 0)
      (Default|StopPushingPulling _playerref))))

(event EventBeginPlay
  (|CallParentFunction) ; This node is disabled and will not be called.\nDrag off pins to build functionality.
)

(event Collision|EventActorBeginOverlap
  (params (OtherActor :type Actor%20Object%20Reference))
  (|CallParentFunction OtherActor) ; This node is disabled and will not be called.\nDrag off pins to build functionality.
)

(event EventTick
  (params (DeltaSeconds :type Float%20%28single-precision%29))
  (|CallParentFunction DeltaSeconds) ; This node is disabled and will not be called.\nDrag off pins to build functionality.
)

(event EventInteraction
  (params (PlayerRef :type Grim%20Dig%20Pawn%20Object%20Reference))
  (if (Math|Float|NearlyEqual(Float) (.z (Transformation|GetActorLocation PlayerRef)) (.z (Transformation|GetActorLocation)) 1e+02)
    (Variables|Default|SetPlayerRef PlayerRef)
    (if (Variables|/Game/Blueprints/Character/GrimDigPawn.GrimDigPawn_C|GetPushingPulling PlayerRef)
      (Variables|/Game/Blueprints/Character/GrimDigPawn.GrimDigPawn_C|SetPushPullBoxRef (Variables|Default|GetPlayerRef) 0)
      (Default|StopPushingPulling (Variables|Default|GetPlayerRef))
      (else
        (Variables|/Game/Blueprints/Character/GrimDigPawn.GrimDigPawn_C|SetPushPullBoxRef (Variables|Default|GetPlayerRef) self)
        (Default|StartPushingPulling (Variables|Default|GetPlayerRef))))
    (else
      (Default|PromptComment PlayerRef "I need to stand just next to it."))))

(fn ConstructionScript
  (|CallParentFunction))

(fn LookforBoxonTop
  (bind _trace (Variables|Default|GetTrace))
  (bind _returnvalue (Transformation|GetWorldLocation _trace))
  (bind _outhit (Collision|LineTraceByChannel (+ _returnvalue "0, 0,-100.000000") (+ _returnvalue "0, 0,100.000000") "TraceTypeQuery1" false 0 "None"))
  (Utilities|IsValid (.hitactor _outhit)
    (:Is%20Valid
      (if (== (Utilities|GetClass (.hitactor _outhit)) "BP_PushPullBox_C")
        (bind _asbp_push_pull_box (Utilities|Casting|CastToBP_PushPullBox (.hitactor _outhit)))
        (Variables|Default|SetBoxOnTop _asbp_push_pull_box)
        (return true)
        (else
          _)))
    (:Is%20Not%20Valid
      _))
  (Variables|Default|SetBoxOnTop 0)
  (return false))