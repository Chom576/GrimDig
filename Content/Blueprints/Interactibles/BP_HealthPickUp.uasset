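; BP_HealthPickUp is an interactible pickup that restores a player's health when used.
; Its Interaction event heals the interacting player by applying negative damage, so healing runs through the standard damage pipeline.
; It then plays a food sound attached to the player's scene component and destroys itself.
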(event EventBeginPlay
  (|CallParentFunction) ; This node is disabled and will not be called.\nDrag off pins to build functionality.
)

(event Collision|EventActorBeginOverlap
  (params (OtherActor :type Actor%20Object%20Reference))
  (|CallParentFunction OtherActor) ; This node is disabled and will not be called.\nDrag off pins to build functionality.
)

(event EventTick
  (params (DeltaSeconds :type Float%20%28single-precision%29))
  (|CallParentFunction DeltaSeconds) ; This node is disabled and will not be called.\nDrag off pins to build functionality.
)

(event EventInteraction
  (params (PlayerRef :type Grim%20Dig%20Pawn%20Object%20Reference))
  (Game|Damage|ApplyDamage PlayerRef -1e+01 0 0)
  (Audio|SpawnSoundAttached "/Game/Assets/Audio/SFX_OGG/Food1_Cue.Food1_Cue" (Variables|/Game/Blueprints/Character/GrimDigPawn.GrimDigPawn_C|GetScene PlayerRef) "None" "0, 0, 0" "0, 0, 0" "KeepRelativeOffset" false 1.0 1.0 0.0 0 0)
  (Actor|DestroyActor))

(fn ConstructionScript
  (|CallParentFunction))