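; BP_CollapseBridge is an interactible bridge that collapses when its Collapse event is called.
; Collapse disables the Box collision and snaps the static mesh to the relative transform of a Scene component, which marks the collapsed pose without animation.
; It then calls EndMovement on the referenced player and clears its CantMove flag.
; Nothing in this Blueprint calls Collapse or sets the player reference.
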(event EventBeginPlay
  (|CallParentFunction) ; This node is disabled and will not be called.\nDrag off pins to build functionality.
)

(event Collision|EventActorBeginOverlap
  (params (OtherActor :type Actor%20Object%20Reference))
  (|CallParentFunction OtherActor) ; This node is disabled and will not be called.\nDrag off pins to build functionality.
)

(event EventTick
  (params (DeltaSeconds :type Float%20%28single-precision%29))
  (|CallParentFunction DeltaSeconds) ; This node is disabled and will not be called.\nDrag off pins to build functionality.
)

(event EventCollapse
  (bind _playerref (Variables|Default|GetPlayerRef))
  (Collision|SetCollisionEnabled (Variables|Default|GetBox) "NoCollision")
  (Transformation|SetRelativeTransform (Variables|Default|GetStaticMesh) (Transformation|GetRelativeTransform (Variables|Default|GetScene)) false false)
  (Default|EndMovement _playerref)
  (Variables|/Game/Blueprints/Character/GrimDigPawn.GrimDigPawn_C|SetCantMove _playerref false))

(fn ConstructionScript
  (|CallParentFunction))