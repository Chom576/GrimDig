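; Base pickup item that a player collects into their inventory by interacting with it.
; The construction script writes the actor's own class into its ItemInfo struct, keeping the other fields intact.
; On Interaction, it asks the player for a free slot, then either adds ItemInfo there, shows a pickup comment and destroys itself, or reports that the inventory is full.
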(event EventBeginPlay
  (|CallParentFunction) ; This node is disabled and will not be called.\nDrag off pins to build functionality.
)

(event Collision|EventActorBeginOverlap
  (params (OtherActor :type Actor%20Object%20Reference))
  (|CallParentFunction OtherActor) ; This node is disabled and will not be called.\nDrag off pins to build functionality.
)

(event EventTick
  (params (DeltaSeconds :type Float%20%28single-precision%29))
  (|CallParentFunction DeltaSeconds) ; This node is disabled and will not be called.\nDrag off pins to build functionality.
)

(event EventInteraction
  (params (PlayerRef :type Grim%20Dig%20Pawn%20Object%20Reference))
  (bind (_hasspace _spacenum) (Default|HasSpaceinInv PlayerRef))
  (if _hasspace
    (Default|AddItem PlayerRef (Variables|Default|GetItemInfo) _spacenum)
    (Default|PromptComment PlayerRef (Utilities|Text|ToText(String) (Utilities|String|Append "You picked up the " (Utilities|String|ToString(Text) (.name (Variables|Default|GetItemInfo))) ".")))
    (Actor|DestroyActor)
    (else
      (Default|PromptComment PlayerRef "Inventory is full."))))

(fn ConstructionScript
  (|CallParentFunction)
  (Variables|Default|SetItemInfo (Utilities|Struct|MakeS_ItemInfo (.name (Variables|Default|GetItemInfo)) (.itemtype (Variables|Default|GetItemInfo)) (.itemimage (Variables|Default|GetItemInfo)) (Utilities|GetClass self) (.stack (Variables|Default|GetItemInfo)) (.quantity (Variables|Default|GetItemInfo)) (.flavour (Variables|Default|GetItemInfo)) (.weight (Variables|Default|GetItemInfo)))))