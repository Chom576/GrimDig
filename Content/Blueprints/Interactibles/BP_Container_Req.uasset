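; BP_Container_Req is an interactable container that switches a linked activable on or off depending on whether it holds a required set of items.
; On each Item event, it matches RequiredItems by class against a temporary copy of its contents, removing and counting matches.
; The inner loop has no break, so one requirement can count several items.
; An exact count match calls TurnOnOpen on ActivableRef; otherwise it calls TurnOffClose.
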(event EventBeginPlay
  (|CallParentFunction) ; This node is disabled and will not be called.\nDrag off pins to build functionality.
)

(event Collision|EventActorBeginOverlap
  (params (OtherActor :type Actor%20Object%20Reference))
  (|CallParentFunction OtherActor) ; This node is disabled and will not be called.\nDrag off pins to build functionality.
)

(event EventTick
  (params (DeltaSeconds :type Float%20%28single-precision%29))
  (|CallParentFunction DeltaSeconds) ; This node is disabled and will not be called.\nDrag off pins to build functionality.
)

(event EventItem
  (params (Slot :type Integer) (ItemInfo :type S%20Item%20Info%20Structure))
  (bind _self self)
  (bind _activableref (Variables|Default|GetActivableRef))
  (|CallParentFunction Slot ItemInfo)
  (Variables|Default|SetReqItemsFound 0)
  (Variables|Default|SetTempContainsTable (Variables|Default|GetContains))
  (for _array_element (Variables|Default|GetRequiredItems)
    (bind (_array_element_2 _array_index) (Utilities|Array|ForEachLoopwithBreak (Variables|Default|GetTempContainsTable))
      (:LoopBody
        (if (== (.ItemClass (Utilities|Struct|BreakS_ItemInfo _array_element_2)) _array_element)
          (Math|Integer|IncrementInt (Variables|Default|GetReqItemsFound)
            (:%20%20
              (Utilities|Array|RemoveIndex (Variables|Default|GetTempContainsTable) _array_index)))))))
  (if (== (Variables|Default|GetReqItemsFound) (Utilities|Array|Length (Variables|Default|GetRequiredItems)))
    (Default|TurnOn/Open _activableref _self)
    (else
      (Default|TurnOff/Close _activableref _self))))

(event EventInteraction
  (params (PlayerRef :type Grim%20Dig%20Pawn%20Object%20Reference))
  (|CallParentFunction PlayerRef))

(fn ConstructionScript
  (|CallParentFunction))