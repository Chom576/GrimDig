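; BP_GoldNugget is an interactable gold pickup that grants gold to the player.
; The PredefGold enum sets mesh scale in the construction script and supplies the amount at BeginPlay unless AmountOfGold already exceeds one.
; A preset amount above one instead picks a coin or bag sound.
; Interaction pays the player, plays the sound, prompts a comment, spawns a burst for larger amounts, then destroys the actor.
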(event EventBeginPlay
  (|CallParentFunction)
  (if (> (Variables|Default|GetAmountOfGold) 1)
    (if (> (Variables|Default|GetAmountOfGold) 15)
      (Variables|Default|SetSoundCue "/Game/Assets/Audio/SFX_OGG/CoinBag1_Cue.CoinBag1_Cue")
      (else
        (Variables|Default|SetSoundCue "/Game/Assets/Audio/SFX_OGG/Coin1_Cue.Coin1_Cue")))
    (else
      (Variables|Default|SetAmountOfGold (Utilities|Select :Index (Variables|Default|GetPredefGold) :NewEnumerator0 1 :NewEnumerator1 3 :NewEnumerator2 15 :NewEnumerator3 50 :NewEnumerator4 200 :NewEnumerator5 500 :NewEnumerator6 1000)))))

(event Collision|EventActorBeginOverlap
  (params (OtherActor :type Actor%20Object%20Reference))
  (|CallParentFunction OtherActor) ; This node is disabled and will not be called.\nDrag off pins to build functionality.
)

(event EventTick
  (params (DeltaSeconds :type Float%20%28single-precision%29))
  (|CallParentFunction DeltaSeconds) ; This node is disabled and will not be called.\nDrag off pins to build functionality.
)

(event EventInteraction
  (params (PlayerRef :type Grim%20Dig%20Pawn%20Object%20Reference))
  (bind _amountofgold (Variables|Default|GetAmountOfGold))
  (Default|GainGold PlayerRef _amountofgold)
  (Audio|SpawnSoundAttached (Variables|Default|GetSoundCue) (Variables|/Game/Blueprints/Character/GrimDigPawn.GrimDigPawn_C|GetScene PlayerRef) "None" "0, 0, 0" "0, 0, 0" "KeepRelativeOffset" false 1.0 1.0 0.0 0 0)
  (Default|PromptComment PlayerRef (Utilities|Text|ToText(String) (Utilities|String|Append "You found " (Utilities|String|ToString(Integer) (Variables|Default|GetAmountOfGold)) (select (> _amountofgold 1) " gold pieces." " gold piece."))))
  (if (> (Variables|Default|GetAmountOfGold) 10)
    (Effects|SpawnEmitteratLocation (Utilities|Select :Index (Variables|Default|GetPredefGold) :NewEnumerator0 0 :NewEnumerator1 0 :NewEnumerator2 "/Game/Assets/ParticleFX/P_NuggetBurst.P_NuggetBurst" :NewEnumerator3 "/Game/Assets/ParticleFX/P_NuggetBurst1.P_NuggetBurst1" :NewEnumerator4 "/Game/Assets/ParticleFX/P_NuggetBurst1.P_NuggetBurst1" :NewEnumerator5 "/Game/Assets/ParticleFX/P_NuggetBurst1.P_NuggetBurst1" :NewEnumerator6 "/Game/Assets/ParticleFX/P_NuggetBurst1.P_NuggetBurst1") (Transformation|GetActorLocation) (Transformation|GetActorRotation)))
  (Actor|DestroyActor))

(fn ConstructionScript
  (bind _predefgold (Variables|Default|GetPredefGold))
  (bind _returnvalue (Utilities|Select :Index _predefgold :NewEnumerator0 0.2 :NewEnumerator1 0.3 :NewEnumerator2 0.5 :NewEnumerator3 1.0 :NewEnumerator4 2.0 :NewEnumerator5 3.0 :NewEnumerator6 5.0))
  (|CallParentFunction)
  (Transformation|SetRelativeScale3D (Variables|Default|GetStaticMesh) (Math|Vector|MakeVector _returnvalue _returnvalue _returnvalue)))