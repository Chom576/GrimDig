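; BP_Container is an interactible item container that the player opens alongside their inventory.
; On BeginPlay it fills Contains with empty slots, writes class defaults from InitialItemList into them, and caches the GrimDigPawn player.
; Interaction toggles the inventory, binds itself and its name to the HUD container widget and shows it.
; ReceiveItem writes an item into a slot and refreshes that widget, while CloseContainer is empty.
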(event Custom|ReceiveItem
  (params (Slot :type Integer) (ItemInfo :type S%20Item%20Info%20Structure))
  (Utilities|Array|SetArrayElem (Variables|Default|GetContains) Slot ItemInfo)
  (Default|RefreshContainer (Variables|/Game/Blueprints/UI/UI_BaseHUD.UI_BaseHUD_C|GetUI_Container (Variables|/Game/Blueprints/Character/GrimDigPawn.GrimDigPawn_C|GetHUD_Ref (Variables|Default|GetPlayerRef)))))

(event Custom|CloseContainer)

(event EventBeginPlay
  (|CallParentFunction)
  (for _index (range 0 (- (Variables|Default|GetSlots) 1))
    (Utilities|Array|Add (Variables|Default|GetContains) (Utilities|Struct|MakeS_ItemInfo "" "NewEnumerator2")))
  (for (_array_element _array_index) (Variables|Default|GetInitialItemList)
    (if (< (- (Utilities|Array|Length (Variables|Default|GetContains)) 1) _array_index)
      (Utilities|Array|Add (Variables|Default|GetContains) (Utilities|GetClassDefaults _array_element)))
    (Utilities|Array|SetArrayElem (Variables|Default|GetContains) _array_index (Utilities|GetClassDefaults _array_element)))
  (bind _asgrim_dig_pawn (Utilities|Casting|CastToGrimDigPawn (Game|Player|GetPlayerPawn 0)))
  (Variables|Default|SetPlayerRef _asgrim_dig_pawn))

(event Collision|EventActorBeginOverlap
  (params (OtherActor :type Actor%20Object%20Reference))
  (|CallParentFunction OtherActor) ; This node is disabled and will not be called.\nDrag off pins to build functionality.
)

(event EventTick
  (params (DeltaSeconds :type Float%20%28single-precision%29))
  (|CallParentFunction DeltaSeconds) ; This node is disabled and will not be called.\nDrag off pins to build functionality.
)

(event EventInteraction
  (params (PlayerRef :type Grim%20Dig%20Pawn%20Object%20Reference))
  (bind _hud_ref (Variables|/Game/Blueprints/Character/GrimDigPawn.GrimDigPawn_C|GetHUD_Ref PlayerRef))
  (bind _ui_container (Variables|/Game/Blueprints/UI/UI_BaseHUD.UI_BaseHUD_C|GetUI_Container _hud_ref))
  (Default|Open/CloseInventory PlayerRef)
  (Variables|/Game/Blueprints/UI/UI_Container.UI_Container_C|SetContainerName _ui_container (Variables|Default|GetContainerName))
  (Variables|/Game/Blueprints/UI/UI_Container.UI_Container_C|SetContainerRef _ui_container self)
  (Variables|/Game/Blueprints/UI/UI_BaseHUD.UI_BaseHUD_C|SetContainerVisibility _hud_ref "Visible")
  (Default|RefreshContainer _ui_container))

(fn ConstructionScript
  (|CallParentFunction))