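; BP_CollapseFloor is a dungeon floor tile that creaks when the GrimDig pawn steps on it and eventually collapses.
; Box overlap locks the pawn's movement, plays a camera shake and dust burst, then checks StepCount after a short delay.
; With steps left, it decrements the count, shows a warning comment, sinks and randomly tilts the mesh, tints it red and frees the pawn.
; At zero, it destroys itself and ends the pawn's movement.
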(event OnComponentBeginOverlap(Box)
  (params (OverlappedComponent :type Primitive%20Component%20Object%20Reference) (OtherActor :type Actor%20Object%20Reference) (OtherComp :type Primitive%20Component%20Object%20Reference) (OtherBodyIndex :type Integer) (bFromSweep :type Boolean) (SweepResult :type Hit%20Result%20Structure%20%28by%20ref%29))
  (bind _returnvalue (Transformation|GetActorLocation))
  (bind _staticmesh (Variables|Default|GetStaticMesh))
  (bind _returnvalue_2 (Transformation|GetRelativeTransform _staticmesh))
  (bind _asgrim_dig_pawn (Utilities|Casting|CastToGrimDigPawn OtherActor))
  (Variables|/Game/Blueprints/Character/GrimDigPawn.GrimDigPawn_C|SetCantMove _asgrim_dig_pawn true)
  (Variables|Default|SetPlayerRef _asgrim_dig_pawn)
  (Camera|PlayWorldCameraShake "/Game/Blueprints/Interactibles/UnstableGround.UnstableGround_C" _returnvalue 0.0 5e+02)
  (Effects|SpawnEmitteratLocation "/Game/Assets/ParticleFX/P_FX_DustFall.P_FX_DustFall" (+ _returnvalue "0, 0,50.000000"))
  (Utilities|FlowControl|Delay 0.5)
  (if (== (Variables|Default|GetStepCount) 0)
    (CallFunction|Collapse)
    (else
      (Math|Integer|DecrementInt (Variables|Default|GetStepCount)
        (:%20%20
          (Default|PromptComment (Variables|Default|GetPlayerRef) "Floor creaks under your feet.")
          (Transformation|SetRelativeTransform _staticmesh (Math|Transform|MakeTransform (+ (.location _returnvalue_2) "0, 0,-10.000000") (Math|Rotator|MakeRotator (Math|Random|RandomFloatinRange -5.0 5.0) (Math|Random|RandomFloatinRange -5.0 5.0) 0.0) (.scale _returnvalue_2)) false false)
          (Variables|/Game/Blueprints/Character/GrimDigPawn.GrimDigPawn_C|SetCantMove (Variables|Default|GetPlayerRef) false)
          (bind _returnvalue_3 (Rendering|Material|CreateDynamicMaterialInstance _staticmesh 0 "/Game/Assets/Materials/Mat_SimpleDungeonsColorCode.Mat_SimpleDungeonsColorCode" "None" :!class /Script/Engine.PrimitiveComponent))
          (Rendering|Material|SetVectorParameterValue _returnvalue_3 "Color" "(R=1.000000,G=0.000000,B=0.000000,A=1.000000)" :!class /Script/Engine.MaterialInstanceDynamic))))))

(event Custom|Collapse
  (bind _playerref (Variables|Default|GetPlayerRef))
  (Actor|DestroyActor)
  (Default|EndMovement _playerref)
  (Variables|/Game/Blueprints/Character/GrimDigPawn.GrimDigPawn_C|SetCantMove _playerref false))

(event EventBeginPlay)

(event Collision|EventActorBeginOverlap
  (params (OtherActor :type Actor%20Object%20Reference)))

(event EventTick
  (params (DeltaSeconds :type Float%20%28single-precision%29)))

(fn ConstructionScript)