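; BP_DragonTrap is an activatable trap that fires a fire projectile when triggered.
; On Activate, it spawns a BP_FireProjectile at its Arrow component's world transform, so the arrow sets the launch point and direction.
; It then copies its HowMuchDamage variable into the new projectile's DamageRating, so damage is set on the trap.
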(event EventBeginPlay
  (|CallParentFunction) ; This node is disabled and will not be called.\nDrag off pins to build functionality.
)

(event Collision|EventActorBeginOverlap
  (params (OtherActor :type Actor%20Object%20Reference))
  (|CallParentFunction OtherActor) ; This node is disabled and will not be called.\nDrag off pins to build functionality.
)

(event EventTick
  (params (DeltaSeconds :type Float%20%28single-precision%29))
  (|CallParentFunction DeltaSeconds) ; This node is disabled and will not be called.\nDrag off pins to build functionality.
)

(event EventActivate
  (params (Initiator :type Actor%20Object%20Reference))
  (bind _returnvalue (Game|SpawnActorfromClass "/Game/Blueprints/Activables/BP_FireProjectile.BP_FireProjectile_C" (Transformation|GetWorldTransform (Variables|Default|GetArrow)) "Undefined" 0 0))
  (Variables|/Game/Blueprints/Activables/BP_FireProjectile.BP_FireProjectile_C|SetDamageRating _returnvalue (Variables|Default|GetHowMuchDamage)))

(fn ConstructionScript
  (|CallParentFunction))