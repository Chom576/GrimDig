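; Activable stone block that slides between Closed and Open component positions when activated, opened or closed, ignoring calls while moving.
; One timeline, played forward or reversed, lerps the block along with its ConnectedActors and any actors stacked on top.
; Stacked actors are found by repeated upward-stepping line traces before each move, with carried actors' endpoints snapped to a 250-unit grid.
; Construction script previews the start state and applies optional color and decal coding.
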(event EventBeginPlay
  (|CallParentFunction)
  (CallFunction|SetStartingEndingLocations)
  (bind _output_get (Variables|Default|SetIsOpen (Variables|Default|GetStartOpen)))
  (if _output_get
    (Transformation|SetRelativeLocation (Variables|Default|GetBlock) (Variables|/Script/Engine.SceneComponent|GetRelativeLocation (Variables|Default|GetOpen)) false false)
    (else
      (Transformation|SetRelativeLocation (Variables|Default|GetBlock) (Variables|/Script/Engine.SceneComponent|GetRelativeLocation (Variables|Default|GetClosed)) false false))))

(event Collision|EventActorBeginOverlap
  (params (OtherActor :type Actor%20Object%20Reference))
  (|CallParentFunction OtherActor) ; This node is disabled and will not be called.\nDrag off pins to build functionality.
)

(event EventTick
  (params (DeltaSeconds :type Float%20%28single-precision%29))
  (|CallParentFunction DeltaSeconds) ; This node is disabled and will not be called.\nDrag off pins to build functionality.
)

(event EventActivate
  (params (Initiator :type Actor%20Object%20Reference))
  (bind _returnvalue (Transformation|GetActorLocation))
  (if (not (Variables|Default|GetIsMoving))
    (if (Variables|Default|GetIsOpen)
      (Variables|Default|SetIsMoving true)
      (Audio|PlaySoundatLocation "/Game/Assets/Audio/SFX_OGG/SFX_-_stone_scrape_02.SFX_-_stone_scrape_02" _returnvalue "0, 0, 0" 1.0 1.0 0.0 "/Game/Assets/Audio/NewSoundAttenuation.NewSoundAttenuation" 0 0)
      (CallFunction|AddActorsonTop)
      (bind (_direction _newtrack_0) (Timeline|Timeline_0 ReverseFromEnd)
        (:Update
          (Transformation|SetRelativeLocation (Variables|Default|GetBlock) (Math|Vector|Lerp(Vector) (Variables|/Script/Engine.SceneComponent|GetRelativeLocation (Variables|Default|GetClosed)) (Variables|/Script/Engine.SceneComponent|GetRelativeLocation (Variables|Default|GetOpen)) _newtrack_0) false false)
          (Utilities|FlowControl|Sequence
            (:then_0
              (for _array_element (Variables|Default|GetConnectedActors)
                (Transformation|SetActorLocation (.WhatActor (Utilities|Struct|BreakMovingBlockStruct _array_element)) (Math|Vector|Lerp(Vector) (.StartingVector (Utilities|Struct|BreakMovingBlockStruct _array_element)) (.EndingVector (Utilities|Struct|BreakMovingBlockStruct _array_element)) _newtrack_0) false false)))
            (:then_1
              (for _array_element_2 (Variables|Default|GetActorsOnTop)
                (Transformation|SetActorLocation (.WhatActor (Utilities|Struct|BreakMovingBlockStruct _array_element_2)) (Math|Vector|Lerp(Vector) (.StartingVector (Utilities|Struct|BreakMovingBlockStruct _array_element_2)) (.EndingVector (Utilities|Struct|BreakMovingBlockStruct _array_element_2)) _newtrack_0) false false)))))
        (:Finished
          (Variables|Default|SetIsMoving false)
          (Variables|Default|SetIsOpen (Utilities|Select :Index _direction :Forward true :Backward false))))
      (else
        (Variables|Default|SetIsMoving true)
        (Audio|PlaySoundatLocation "/Game/Assets/Audio/SFX_OGG/SFX_-_stone_scrape_02.SFX_-_stone_scrape_02" _returnvalue "0, 0, 0" 1.0 1.0 0.0 "/Game/Assets/Audio/NewSoundAttenuation.NewSoundAttenuation" 0 0)
        (CallFunction|AddActorsonTop)
        (Timeline|Timeline_0 PlayFromStart)))))

(event EventTurnOff/Close
  (params (Initiator :type Actor%20Object%20Reference))
  (if (not (Variables|Default|GetIsMoving))
    (if (Variables|Default|GetIsOpen)
      (Variables|Default|SetIsMoving true)
      (Audio|PlaySoundatLocation "/Game/Assets/Audio/SFX_OGG/SFX_-_stone_scrape_02.SFX_-_stone_scrape_02" (Transformation|GetActorLocation) "0, 0, 0" 1.0 1.0 0.0 "/Game/Assets/Audio/NewSoundAttenuation.NewSoundAttenuation" 0 0)
      (CallFunction|AddActorsonTop)
      (bind (_direction _newtrack_0) (Timeline|Timeline_0 ReverseFromEnd)
        (:Update
          (Transformation|SetRelativeLocation (Variables|Default|GetBlock) (Math|Vector|Lerp(Vector) (Variables|/Script/Engine.SceneComponent|GetRelativeLocation (Variables|Default|GetClosed)) (Variables|/Script/Engine.SceneComponent|GetRelativeLocation (Variables|Default|GetOpen)) _newtrack_0) false false)
          (Utilities|FlowControl|Sequence
            (:then_0
              (for _array_element (Variables|Default|GetConnectedActors)
                (Transformation|SetActorLocation (.WhatActor (Utilities|Struct|BreakMovingBlockStruct _array_element)) (Math|Vector|Lerp(Vector) (.StartingVector (Utilities|Struct|BreakMovingBlockStruct _array_element)) (.EndingVector (Utilities|Struct|BreakMovingBlockStruct _array_element)) _newtrack_0) false false)))
            (:then_1
              (for _array_element_2 (Variables|Default|GetActorsOnTop)
                (Transformation|SetActorLocation (.WhatActor (Utilities|Struct|BreakMovingBlockStruct _array_element_2)) (Math|Vector|Lerp(Vector) (.StartingVector (Utilities|Struct|BreakMovingBlockStruct _array_element_2)) (.EndingVector (Utilities|Struct|BreakMovingBlockStruct _array_element_2)) _newtrack_0) false false)))))
        (:Finished
          (Variables|Default|SetIsMoving false)
          (Variables|Default|SetIsOpen (Utilities|Select :Index _direction :Forward true :Backward false)))))))

(event EventTurnOn/Open
  (params (Initiator :type Actor%20Object%20Reference))
  (if (not (Variables|Default|GetIsMoving))
    (if (not (Variables|Default|GetIsOpen))
      (Variables|Default|SetIsMoving true)
      (Audio|PlaySoundatLocation "/Game/Assets/Audio/SFX_OGG/SFX_-_stone_scrape_02.SFX_-_stone_scrape_02" (Transformation|GetActorLocation) "0, 0, 0" 1.0 1.0 0.0 "/Game/Assets/Audio/NewSoundAttenuation.NewSoundAttenuation" 0 0)
      (CallFunction|AddActorsonTop)
      (bind (_direction _newtrack_0) (Timeline|Timeline_0 PlayFromStart)
        (:Update
          (Transformation|SetRelativeLocation (Variables|Default|GetBlock) (Math|Vector|Lerp(Vector) (Variables|/Script/Engine.SceneComponent|GetRelativeLocation (Variables|Default|GetClosed)) (Variables|/Script/Engine.SceneComponent|GetRelativeLocation (Variables|Default|GetOpen)) _newtrack_0) false false)
          (Utilities|FlowControl|Sequence
            (:then_0
              (for _array_element (Variables|Default|GetConnectedActors)
                (Transformation|SetActorLocation (.WhatActor (Utilities|Struct|BreakMovingBlockStruct _array_element)) (Math|Vector|Lerp(Vector) (.StartingVector (Utilities|Struct|BreakMovingBlockStruct _array_element)) (.EndingVector (Utilities|Struct|BreakMovingBlockStruct _array_element)) _newtrack_0) false false)))
            (:then_1
              (for _array_element_2 (Variables|Default|GetActorsOnTop)
                (Transformation|SetActorLocation (.WhatActor (Utilities|Struct|BreakMovingBlockStruct _array_element_2)) (Math|Vector|Lerp(Vector) (.StartingVector (Utilities|Struct|BreakMovingBlockStruct _array_element_2)) (.EndingVector (Utilities|Struct|BreakMovingBlockStruct _array_element_2)) _newtrack_0) false false)))))
        (:Finished
          (Variables|Default|SetIsMoving false)
          (Variables|Default|SetIsOpen (Utilities|Select :Index _direction :Forward true :Backward false)))))))

(fn ConstructionScript
  (|CallParentFunction)
  (if (Variables|Default|GetColorCoded?)
    (bind _returnvalue (Rendering|Material|CreateDynamicMaterialInstance (Variables|Default|GetBlock) 0 "/Game/Assets/Materials/SimpleTempleColorCode.SimpleTempleColorCode" "None" :!class /Script/Engine.PrimitiveComponent))
    (Rendering|Material|SetVectorParameterValue _returnvalue "Color" (Variables|Default|GetColorCode) :!class /Script/Engine.MaterialInstanceDynamic))
  (if (Variables|Default|GetDecalCoded?)
    (for _array_element (Actor|GetComponentsbyTag "/Script/Engine.DecalComponent" "Code")
      (bind _returnvalue_2 (Rendering|Material|CreateDynamicMaterialInstance _array_element :!class /Script/Engine.DecalComponent))
      (Rendering|Material|SetTextureParameterValue _returnvalue_2 "Icon" (Variables|Default|GetDecalIcon))
      (Rendering|Material|SetVectorParameterValue _returnvalue_2 "Color" (Variables|Default|GetDecalColor) :!class /Script/Engine.MaterialInstanceDynamic)
      (Rendering|SetVisibility _array_element true false)))
  (bind _output_get (Variables|Default|SetIsOpen (Variables|Default|GetStartOpen)))
  (if _output_get
    (Transformation|SetRelativeLocation (Variables|Default|GetBlock) (Variables|/Script/Engine.SceneComponent|GetRelativeLocation (Variables|Default|GetOpen)) false false)
    (else
      (Transformation|SetRelativeLocation (Variables|Default|GetBlock) (Variables|/Script/Engine.SceneComponent|GetRelativeLocation (Variables|Default|GetClosed)) false false))))

(fn SetStartingEndingLocations
  (bind _connectedactors (Variables|Default|GetConnectedActors))
  (for (_array_element _array_index) _connectedactors
    (Utilities|Array|SetArrayElem _connectedactors _array_index (Utilities|MakeStartingEndingVector (.WhatActor (Utilities|Struct|BreakMovingBlockStruct _array_element)))))
  (return))

(fn AddActorsonTop
  (Utilities|Array|Clear (Variables|Default|GetActorsToIgnore))
  (Utilities|Array|Clear (Variables|Default|GetActorsOnTop))
  (LocalVariables|SetTempTracePoint (Transformation|GetWorldLocation (Variables|Default|GetTracePoint)))
  (bind (_outhit _returnvalue) (Collision|LineTraceByChannel (+ (LocalVariables|GetTempTracePoint) "0, 0,-100.000000") (+ (LocalVariables|GetTempTracePoint) "0, 0,100.000000") "TraceTypeQuery1" false (Variables|Default|GetActorsToIgnore) "None" :!label _label))
  (if _returnvalue
    (Utilities|Array|Add (Variables|Default|GetActorsOnTop) (Utilities|MakeStartingEndingVector (.HitActor (Collision|BreakHitResult _outhit))))
    (Utilities|Array|Add (Variables|Default|GetActorsToIgnore) (.HitActor (Collision|BreakHitResult _outhit)))
    (Development|PrintString (Utilities|GetDisplayName (.HitActor (Collision|BreakHitResult _outhit))))
    (LocalVariables|SetTempTracePoint (+ (LocalVariables|GetTempTracePoint) "0,0.000000,500.000000"))
    (goto _label)
    (else
      (return))))