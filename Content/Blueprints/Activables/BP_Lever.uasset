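; Lever puzzle switch that the player pulls by direct interaction or by whip, the latter only when standing near its grid-snapped valid start point.
; A timeline slides the handle between Start and End, flags player movement as in progress, and blocks retriggering until finished.
; A timeline event track signals the actors in the turn-on, turn-off and activate lists.
; The construction script optionally tints handle and base with a color-code material.
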(event EventBeginPlay
  (|CallParentFunction) ; This node is disabled and will not be called.\nDrag off pins to build functionality.
)

(event Collision|EventActorBeginOverlap
  (params (OtherActor :type Actor%20Object%20Reference))
  (|CallParentFunction OtherActor) ; This node is disabled and will not be called.\nDrag off pins to build functionality.
)

(event EventTick
  (params (DeltaSeconds :type Float%20%28single-precision%29))
  (|CallParentFunction DeltaSeconds) ; This node is disabled and will not be called.\nDrag off pins to build functionality.
)

(event EventInteraction
  (params (PlayerRef :type Grim%20Dig%20Pawn%20Object%20Reference))
  (bind _turnonlist (Variables|Default|GetTurnOnList))
  (bind _turnofflist (Variables|Default|GetTurnOffList))
  (bind _activatelist (Variables|Default|GetActivateList))
  (Variables|Default|SetPlayerRef PlayerRef)
  (Variables|/Game/Blueprints/Character/GrimDigPawn.GrimDigPawn_C|SetMovementInProgress (Variables|Default|GetPlayerRef) true)
  (if (not (Variables|Default|GetAnimInProgress))
    (Variables|Default|SetAnimInProgress true)
    (Audio|PlaySoundatLocation "/Game/Assets/Audio/SFX_OGG/SFX_-_wood_scrape_02.SFX_-_wood_scrape_02" (Transformation|GetActorLocation) "0, 0, 0" 1.0 1.0 0.0 "/Game/Assets/Audio/NewSoundAttenuation.NewSoundAttenuation" 0 0)
    (bind _newtrack_0 (Timeline|Timeline_0 PlayFromStart)
      (:Update
        (Transformation|SetRelativeLocation (Variables|Default|GetHandle) (Math|Vector|Lerp(Vector) (Variables|/Script/Engine.SceneComponent|GetRelativeLocation (Variables|Default|GetStart)) (Variables|/Script/Engine.SceneComponent|GetRelativeLocation (Variables|Default|GetEnd)) _newtrack_0) false false))
      (:Finished
        (Variables|Default|SetAnimInProgress false)
        (Variables|/Game/Blueprints/Character/GrimDigPawn.GrimDigPawn_C|SetMovementInProgress (Variables|Default|GetPlayerRef) false)
        (if (Variables|Default|GetWhipped?)
          (Default|WhipCableHide (Variables|Default|GetPlayerRef))
          (Variables|Default|SetWhipped? false)))
      (:NewTrack_2
        (if (> (Utilities|Array|Length _turnonlist) 0)
          (for _array_element _turnonlist
            (Utilities|IsValid _array_element
              (:Is%20Valid
                (Default|TurnOn/Open _array_element self)))))
        (if (> (Utilities|Array|Length _turnofflist) 0)
          (for _array_element_2 _turnofflist
            (Utilities|IsValid _array_element_2
              (:Is%20Valid
                (Default|TurnOff/Close _array_element_2 self)))))
        (if (> (Utilities|Array|Length _activatelist) 0)
          (for _array_element_3 _activatelist
            (Utilities|IsValid _array_element_3
              (:Is%20Valid
                (Default|Activate _array_element_3 self)))))))))

(event EventWhipInteract
  (params (PlayerRef :type Grim%20Dig%20Pawn%20Object%20Reference))
  (bind _turnonlist (Variables|Default|GetTurnOnList))
  (bind _turnofflist (Variables|Default|GetTurnOffList))
  (bind _activatelist (Variables|Default|GetActivateList))
  (Variables|Default|SetPlayerRef PlayerRef)
  (if (Math|Vector|Equal(Vector) (Transformation|GetActorLocation (Variables|Default|GetPlayerRef)) (Class|KismetMathLibrary|VectorSnappedtoGrid (Transformation|GetWorldLocation (Variables|Default|GetValidStartPoint)) 2.5e+02) 5e+02)
    (Variables|Default|SetWhipped? true)
    (Default|WhipCableShowUp (Variables|Default|GetPlayerRef))
    (Variables|/Game/Blueprints/Character/GrimDigPawn.GrimDigPawn_C|SetMovementInProgress (Variables|Default|GetPlayerRef) true)
    (if (not (Variables|Default|GetAnimInProgress))
      (Variables|Default|SetAnimInProgress true)
      (Audio|PlaySoundatLocation "/Game/Assets/Audio/SFX_OGG/SFX_-_wood_scrape_02.SFX_-_wood_scrape_02" (Transformation|GetActorLocation) "0, 0, 0" 1.0 1.0 0.0 "/Game/Assets/Audio/NewSoundAttenuation.NewSoundAttenuation" 0 0)
      (bind _newtrack_0 (Timeline|Timeline_0 PlayFromStart)
        (:Update
          (Transformation|SetRelativeLocation (Variables|Default|GetHandle) (Math|Vector|Lerp(Vector) (Variables|/Script/Engine.SceneComponent|GetRelativeLocation (Variables|Default|GetStart)) (Variables|/Script/Engine.SceneComponent|GetRelativeLocation (Variables|Default|GetEnd)) _newtrack_0) false false))
        (:Finished
          (Variables|Default|SetAnimInProgress false)
          (Variables|/Game/Blueprints/Character/GrimDigPawn.GrimDigPawn_C|SetMovementInProgress (Variables|Default|GetPlayerRef) false)
          (if (Variables|Default|GetWhipped?)
            (Default|WhipCableHide (Variables|Default|GetPlayerRef))
            (Variables|Default|SetWhipped? false)))
        (:NewTrack_2
          (if (> (Utilities|Array|Length _turnonlist) 0)
            (for _array_element _turnonlist
              (Utilities|IsValid _array_element
                (:Is%20Valid
                  (Default|TurnOn/Open _array_element self)))))
          (if (> (Utilities|Array|Length _turnofflist) 0)
            (for _array_element_2 _turnofflist
              (Utilities|IsValid _array_element_2
                (:Is%20Valid
                  (Default|TurnOff/Close _array_element_2 self)))))
          (if (> (Utilities|Array|Length _activatelist) 0)
            (for _array_element_3 _activatelist
              (Utilities|IsValid _array_element_3
                (:Is%20Valid
                  (Default|Activate _array_element_3 self))))))))
    (else
      (Default|PromptComment (Variables|Default|GetPlayerRef) "I can't whip it from this angle."))))

(fn ConstructionScript
  (|CallParentFunction)
  (if (Variables|Default|GetColorCoded?)
    (bind _returnvalue (Rendering|Material|CreateDynamicMaterialInstance (Variables|Default|GetHandle) 0 "/Game/Assets/Materials/SimpleTempleColorCode.SimpleTempleColorCode" "None" :!class /Script/Engine.PrimitiveComponent))
    (Rendering|Material|SetVectorParameterValue _returnvalue "Color" (Variables|Default|GetColorCode) :!class /Script/Engine.MaterialInstanceDynamic)
    (bind _returnvalue_2 (Rendering|Material|CreateDynamicMaterialInstance (Variables|Default|GetStaticMesh) 0 "/Game/Assets/Materials/SimpleTempleColorCode.SimpleTempleColorCode" "None" :!class /Script/Engine.PrimitiveComponent))
    (Rendering|Material|SetVectorParameterValue _returnvalue_2 "Color" (Variables|Default|GetColorCode) :!class /Script/Engine.MaterialInstanceDynamic)))