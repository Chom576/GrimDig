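; Activable sliding door that can be toggled, opened or closed through Activate, TurnOn/Open and TurnOff/Close events.
; A timeline lerps the doorway mesh between Open and Closed component locations with a stone scrape sound, ignoring new triggers while moving.
; The construction script previews the StartOpen position and optionally applies a color-coded dynamic material, plus a tinted icon decal when color coding is on.
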(event EventBeginPlay
  (|CallParentFunction)
  (bind _output_get (Variables|Default|SetIsOpen (Variables|Default|GetStartOpen)))
  (if _output_get
    (Transformation|SetRelativeLocation (Variables|Default|GetSM_Env_Doorway_Simple_01) (Variables|/Script/Engine.SceneComponent|GetRelativeLocation (Variables|Default|GetOpen)) false false)
    (else
      (Transformation|SetRelativeLocation (Variables|Default|GetSM_Env_Doorway_Simple_01) (Variables|/Script/Engine.SceneComponent|GetRelativeLocation (Variables|Default|GetClosed)) false false))))

(event Collision|EventActorBeginOverlap
  (params (OtherActor :type Actor%20Object%20Reference))
  (|CallParentFunction OtherActor) ; This node is disabled and will not be called.\nDrag off pins to build functionality.
)

(event EventTick
  (params (DeltaSeconds :type Float%20%28single-precision%29))
  (|CallParentFunction DeltaSeconds) ; This node is disabled and will not be called.\nDrag off pins to build functionality.
)

(event EventActivate
  (params (Initiator :type Actor%20Object%20Reference))
  (bind _returnvalue (Transformation|GetActorLocation))
  (if (not (Variables|Default|GetIsMoving))
    (if (Variables|Default|GetIsOpen)
      (Variables|Default|SetIsMoving true)
      (Audio|PlaySoundatLocation "/Game/Assets/Audio/SFX_OGG/SFX_-_stone_scrape_02.SFX_-_stone_scrape_02" _returnvalue "0, 0, 0" 1.0 1.0 0.0 "/Game/Assets/Audio/NewSoundAttenuation.NewSoundAttenuation" 0 0)
      (bind (_direction _newtrack_0) (Timeline|Timeline_0 ReverseFromEnd)
        (:Update
          (Transformation|SetRelativeLocation (Variables|Default|GetSM_Env_Doorway_Simple_01) (Math|Vector|Lerp(Vector) (Variables|/Script/Engine.SceneComponent|GetRelativeLocation (Variables|Default|GetClosed)) (Variables|/Script/Engine.SceneComponent|GetRelativeLocation (Variables|Default|GetOpen)) _newtrack_0) false false))
        (:Finished
          (Variables|Default|SetIsMoving false)
          (Variables|Default|SetIsOpen (Utilities|Select :Index _direction :Forward true :Backward false))))
      (else
        (Variables|Default|SetIsMoving true)
        (Audio|PlaySoundatLocation "/Game/Assets/Audio/SFX_OGG/SFX_-_stone_scrape_02.SFX_-_stone_scrape_02" _returnvalue "0, 0, 0" 1.0 1.0 0.0 "/Game/Assets/Audio/NewSoundAttenuation.NewSoundAttenuation" 0 0)
        (Timeline|Timeline_0 PlayFromStart)))))

(event EventTurnOff/Close
  (params (Initiator :type Actor%20Object%20Reference))
  (if (not (Variables|Default|GetIsMoving))
    (if (Variables|Default|GetIsOpen)
      (Variables|Default|SetIsMoving true)
      (Audio|PlaySoundatLocation "/Game/Assets/Audio/SFX_OGG/SFX_-_stone_scrape_02.SFX_-_stone_scrape_02" (Transformation|GetActorLocation) "0, 0, 0" 1.0 1.0 0.0 "/Game/Assets/Audio/NewSoundAttenuation.NewSoundAttenuation" 0 0)
      (bind (_direction _newtrack_0) (Timeline|Timeline_0 ReverseFromEnd)
        (:Update
          (Transformation|SetRelativeLocation (Variables|Default|GetSM_Env_Doorway_Simple_01) (Math|Vector|Lerp(Vector) (Variables|/Script/Engine.SceneComponent|GetRelativeLocation (Variables|Default|GetClosed)) (Variables|/Script/Engine.SceneComponent|GetRelativeLocation (Variables|Default|GetOpen)) _newtrack_0) false false))
        (:Finished
          (Variables|Default|SetIsMoving false)
          (Variables|Default|SetIsOpen (Utilities|Select :Index _direction :Forward true :Backward false)))))))

(event EventTurnOn/Open
  (params (Initiator :type Actor%20Object%20Reference))
  (if (not (Variables|Default|GetIsMoving))
    (if (not (Variables|Default|GetIsOpen))
      (Variables|Default|SetIsMoving true)
      (Audio|PlaySoundatLocation "/Game/Assets/Audio/SFX_OGG/SFX_-_stone_scrape_02.SFX_-_stone_scrape_02" (Transformation|GetActorLocation) "0, 0, 0" 1.0 1.0 0.0 "/Game/Assets/Audio/NewSoundAttenuation.NewSoundAttenuation" 0 0)
      (bind (_direction _newtrack_0) (Timeline|Timeline_0 PlayFromStart)
        (:Update
          (Transformation|SetRelativeLocation (Variables|Default|GetSM_Env_Doorway_Simple_01) (Math|Vector|Lerp(Vector) (Variables|/Script/Engine.SceneComponent|GetRelativeLocation (Variables|Default|GetClosed)) (Variables|/Script/Engine.SceneComponent|GetRelativeLocation (Variables|Default|GetOpen)) _newtrack_0) false false))
        (:Finished
          (Variables|Default|SetIsMoving false)
          (Variables|Default|SetIsOpen (Utilities|Select :Index _direction :Forward true :Backward false)))))))

(fn ConstructionScript
  (|CallParentFunction)
  (if (Variables|Default|GetColorCoded?)
    (bind _returnvalue (Rendering|Material|CreateDynamicMaterialInstance (Variables|Default|GetSM_Env_Doorway_Simple_01) 0 "/Game/Assets/Materials/SimpleTempleColorCode.SimpleTempleColorCode" "None" :!class /Script/Engine.PrimitiveComponent))
    (Rendering|Material|SetVectorParameterValue _returnvalue "Color" (Variables|Default|GetColorCode) :!class /Script/Engine.MaterialInstanceDynamic)
    (if (Variables|Default|GetDecalCoded?)
      (bind _returnvalue_2 (Rendering|Material|CreateDynamicMaterialInstance (Variables|Default|GetDecal) :!class /Script/Engine.DecalComponent))
      (Rendering|Material|SetTextureParameterValue _returnvalue_2 "Icon" (Variables|Default|GetDecalIcon))
      (Rendering|Material|SetVectorParameterValue _returnvalue_2 "Color" (Variables|Default|GetDecalColor) :!class /Script/Engine.MaterialInstanceDynamic)
      (Rendering|SetVisibility (Variables|Default|GetDecal) true false)))
  (bind _output_get (Variables|Default|SetIsOpen (Variables|Default|GetStartOpen)))
  (if _output_get
    (Transformation|SetRelativeLocation (Variables|Default|GetSM_Env_Doorway_Simple_01) (Variables|/Script/Engine.SceneComponent|GetRelativeLocation (Variables|Default|GetOpen)) false false)
    (else
      (Transformation|SetRelativeLocation (Variables|Default|GetSM_Env_Doorway_Simple_01) (Variables|/Script/Engine.SceneComponent|GetRelativeLocation (Variables|Default|GetClosed)) false false))))