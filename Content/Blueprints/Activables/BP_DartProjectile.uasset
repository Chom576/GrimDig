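; BP_DartProjectile is a dart projectile that damages the GrimDig player pawn on overlap.
; Its box overlap applies DamageRating to a living player and destroys the dart at once.
; Other overlaps stop its projectile movement after a tiny delay and destroy it a second later.
; An Indestruct flag, cleared shortly after BeginPlay, lets it ignore those non-player overlaps at launch.
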(event OnComponentBeginOverlap(Box)
  (params (OverlappedComponent :type Primitive%20Component%20Object%20Reference) (OtherActor :type Actor%20Object%20Reference) (OtherComp :type Primitive%20Component%20Object%20Reference) (OtherBodyIndex :type Integer) (bFromSweep :type Boolean) (SweepResult :type Hit%20Result%20Structure%20%28by%20ref%29))
  (bind _asgrim_dig_pawn (Utilities|Casting|CastToGrimDigPawn OtherActor)
    (:then
      (if (not (Variables|/Game/Blueprints/Character/GrimDigPawn.GrimDigPawn_C|GetPlayerDead _asgrim_dig_pawn))
        (Game|Damage|ApplyDamage _asgrim_dig_pawn (Variables|Default|GetDamageRating) 0 0)
        (Actor|DestroyActor)))
    (:CastFailed
      (if (not (Variables|Default|GetIndestruct))
        (Utilities|FlowControl|Delay 0.02)
        (Components|Movement|StopMovementImmediately (Variables|Default|GetProjectileMovement))
        (Utilities|FlowControl|Delay 1.0)
        (Actor|DestroyActor)))))

(event EventBeginPlay
  (Utilities|FlowControl|Delay 0.2)
  (Variables|Default|SetIndestruct false))

(event Collision|EventActorBeginOverlap
  (params (OtherActor :type Actor%20Object%20Reference)))

(event EventTick
  (params (DeltaSeconds :type Float%20%28single-precision%29)))

(fn ConstructionScript)