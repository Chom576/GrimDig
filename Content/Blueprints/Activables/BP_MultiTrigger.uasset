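; Multi-input logic gate activable that switches its linked targets based on whether every actor in RequiredTriggers has signalled it.
; TurnOn/Open adds the caller to InitiatorList, TurnOff/Close removes it, and Activate toggles it, then each rechecks the required set.
; A complete set turns on TurnOnList, while an incomplete one turns off TurnOffList.
; BeginPlay fires TurnOnOpen without an initiator, and membership tests only count indices above zero.
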(event Custom|AllTriggersPresent
  (bind _turnonlist (Variables|Default|GetTurnOnList))
  (if (> (Utilities|Array|Length _turnonlist) 0)
    (for _array_element _turnonlist
      (Utilities|IsValid _array_element
        (:Is%20Valid
          (Default|TurnOn/Open _array_element self))))))

(event Custom|NotEnoughTriggers
  (bind _turnofflist (Variables|Default|GetTurnOffList))
  (if (> (Utilities|Array|Length _turnofflist) 0)
    (for _array_element _turnofflist
      (Utilities|IsValid _array_element
        (:Is%20Valid
          (Default|TurnOff/Close _array_element self))))))

(event Custom|ActivateTheList
  (bind _activatelist (Variables|Default|GetActivateList))
  (if (> (Utilities|Array|Length _activatelist) 0)
    (for _array_element _activatelist
      (Utilities|IsValid _array_element
        (:Is%20Valid
          (Default|Activate _array_element self))))))

(event EventBeginPlay
  (|CallParentFunction)
  (if true
    (CallFunction|TurnOn/Open)))

(event Collision|EventActorBeginOverlap
  (params (OtherActor :type Actor%20Object%20Reference))
  (|CallParentFunction OtherActor) ; This node is disabled and will not be called.\nDrag off pins to build functionality.
)

(event EventTick
  (params (DeltaSeconds :type Float%20%28single-precision%29))
  (|CallParentFunction DeltaSeconds) ; This node is disabled and will not be called.\nDrag off pins to build functionality.
)

(event EventActivate
  (params (Initiator :type Actor%20Object%20Reference))
  (bind _initiatorlist (Variables|Default|GetInitiatorList))
  (if (> (Utilities|Array|FindItem _initiatorlist Initiator) 0)
    (Utilities|Array|RemoveItem (Variables|Default|GetInitiatorList) (stale EventTurnOff/Close Initiator))
    (else
      (Utilities|Array|AddUnique _initiatorlist (stale EventTurnOn/Open Initiator))))
  (Variables|Default|SetFound%20Missing%20Trigger false)
  (bind _array_element (Utilities|Array|ForEachLoopwithBreak (Variables|Default|GetRequiredTriggers) :!label _label)
    (:LoopBody
      (if (not (> (Utilities|Array|FindItem (Variables|Default|GetInitiatorList) _array_element) 0))
        (Variables|Default|SetFound%20Missing%20Trigger true)
        (goto _label Break)))
    (:Completed
      (if (Variables|Default|GetFound%20Missing%20Trigger)
        (CallFunction|NotEnoughTriggers)
        (else
          (CallFunction|AllTriggersPresent))))))

(event EventTurnOff/Close
  (params (Initiator :type Actor%20Object%20Reference))
  (Utilities|Array|RemoveItem (Variables|Default|GetInitiatorList) Initiator)
  (Variables|Default|SetFound%20Missing%20Trigger false)
  (bind _array_element (Utilities|Array|ForEachLoopwithBreak (Variables|Default|GetRequiredTriggers) :!label _label)
    (:LoopBody
      (if (not (> (Utilities|Array|FindItem (Variables|Default|GetInitiatorList) _array_element) 0))
        (Variables|Default|SetFound%20Missing%20Trigger true)
        (goto _label Break)))
    (:Completed
      (if (Variables|Default|GetFound%20Missing%20Trigger)
        (CallFunction|NotEnoughTriggers)
        (else
          (CallFunction|AllTriggersPresent))))))

(event EventTurnOn/Open
  (params (Initiator :type Actor%20Object%20Reference))
  (Utilities|Array|AddUnique (Variables|Default|GetInitiatorList) Initiator)
  (Variables|Default|SetFound%20Missing%20Trigger false)
  (bind _array_element (Utilities|Array|ForEachLoopwithBreak (Variables|Default|GetRequiredTriggers) :!label _label)
    (:LoopBody
      (if (not (> (Utilities|Array|FindItem (Variables|Default|GetInitiatorList) _array_element) 0))
        (Variables|Default|SetFound%20Missing%20Trigger true)
        (goto _label Break)))
    (:Completed
      (if (Variables|Default|GetFound%20Missing%20Trigger)
        (CallFunction|NotEnoughTriggers)
        (else
          (CallFunction|AllTriggersPresent))))))

(fn ConstructionScript
  (|CallParentFunction))