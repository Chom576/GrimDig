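; Activable timer that, on expiry, triggers other objects through its TurnOn, TurnOff and Activate lists.
; It can start on BeginPlay or via TurnOn/Open, TurnOff/Close clears it, and Activate toggles it.
; A timer event, optionally looping, calls the matching action on each valid list entry.
; TimerRunning guards start and stop, and stays true after expiry until the timer is turned off or toggled.
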(event Custom|Timer%20Finished
  (bind _turnonlist (Variables|Default|GetTurnOnList))
  (bind _turnofflist (Variables|Default|GetTurnOffList))
  (bind _activatelist (Variables|Default|GetActivateList))
  (if (> (Utilities|Array|Length _turnonlist) 0)
    (for _array_element _turnonlist
      (Utilities|IsValid _array_element
        (:Is%20Valid
          (Default|TurnOn/Open _array_element)))))
  (if (> (Utilities|Array|Length _turnofflist) 0)
    (for _array_element_2 _turnofflist
      (Utilities|IsValid _array_element_2
        (:Is%20Valid
          (Default|TurnOff/Close _array_element_2)))))
  (if (> (Utilities|Array|Length _activatelist) 0)
    (for _array_element_3 _activatelist
      (Utilities|IsValid _array_element_3
        (:Is%20Valid
          (Default|Activate _array_element_3))))))

(event EventBeginPlay
  (|CallParentFunction)
  (if (Variables|Default|GetStartOn?)
    (bind _returnvalue (Utilities|Time|SetTimerbyEvent (delegate Custom|Timer%20Finished) (Variables|Default|GetTimer) (Variables|Default|GetLooping)))
    (Variables|Default|SetTimerRunning? true)))

(event Collision|EventActorBeginOverlap
  (params (OtherActor :type Actor%20Object%20Reference))
  (|CallParentFunction OtherActor) ; This node is disabled and will not be called.\nDrag off pins to build functionality.
)

(event EventTick
  (params (DeltaSeconds :type Float%20%28single-precision%29))
  (|CallParentFunction DeltaSeconds) ; This node is disabled and will not be called.\nDrag off pins to build functionality.
)

(event EventActivate
  (params (Initiator :type Actor%20Object%20Reference))
  (if (Variables|Default|GetTimerRunning?)
    (Utilities|Time|ClearandInvalidateTimerbyHandle (stale _returnvalue))
    (Variables|Default|SetTimerRunning? false)
    (else
      (bind _returnvalue (Utilities|Time|SetTimerbyEvent (delegate Custom|Timer%20Finished) (Variables|Default|GetTimer) (Variables|Default|GetLooping)))
      (Variables|Default|SetTimerRunning? true))))

(event EventTurnOff/Close
  (params (Initiator :type Actor%20Object%20Reference))
  (if (Variables|Default|GetTimerRunning?)
    (Utilities|Time|ClearandInvalidateTimerbyHandle (stale EventBeginPlay _returnvalue))
    (Variables|Default|SetTimerRunning? false)))

(event EventTurnOn/Open
  (params (Initiator :type Actor%20Object%20Reference))
  (if (not (Variables|Default|GetTimerRunning?))
    (bind _returnvalue (Utilities|Time|SetTimerbyEvent (delegate Custom|Timer%20Finished) (Variables|Default|GetTimer) (Variables|Default|GetLooping)))
    (Variables|Default|SetTimerRunning? true)))

(fn ConstructionScript
  (|CallParentFunction))