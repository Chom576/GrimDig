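; BP_AutoTorch is an activable torch that can be lit or put out through events inherited from its activable interface or parent.
; TurnOn/Open and TurnOff/Close show or hide the point light and particle system together and track the state in Alight.
; Activate toggles between those two states based on Alight.
; The construction script lights the torch when StartOn is set.
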(event EventBeginPlay
  (|CallParentFunction))

(event Collision|EventActorBeginOverlap
  (params (OtherActor :type Actor%20Object%20Reference))
  (|CallParentFunction OtherActor) ; This node is disabled and will not be called.\nDrag off pins to build functionality.
)

(event EventTick
  (params (DeltaSeconds :type Float%20%28single-precision%29))
  (|CallParentFunction DeltaSeconds) ; This node is disabled and will not be called.\nDrag off pins to build functionality.
)

(event EventActivate
  (params (Initiator :type Actor%20Object%20Reference))
  (if (Variables|Default|GetAlight?)
    (Rendering|SetVisibility (Variables|Default|GetParticleSystem) false false)
    (Variables|Default|SetAlight? false)
    (else
      (Rendering|SetVisibility (Variables|Default|GetPointLight) true false)
      (Variables|Default|SetAlight? true))))

(event EventTurnOn/Open
  (params (Initiator :type Actor%20Object%20Reference))
  (Rendering|SetVisibility (Variables|Default|GetPointLight) true false)
  (Variables|Default|SetAlight? true))

(event EventTurnOff/Close
  (params (Initiator :type Actor%20Object%20Reference))
  (Rendering|SetVisibility (Variables|Default|GetParticleSystem) false false)
  (Variables|Default|SetAlight? false))

(fn ConstructionScript
  (|CallParentFunction)
  (if (Variables|Default|GetStartOn?)
    (CallFunction|TurnOn/Open)))