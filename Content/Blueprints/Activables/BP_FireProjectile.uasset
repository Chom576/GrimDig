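; BP_FireProjectile is a fire projectile that damages a living GrimDigPawn on overlap with its box.
; On that hit it stops moving, disables its fire emitter, zeroes its light via a timeline, spawns a smoke ring and destroys itself after a delay.
; Other overlaps trigger the same shutdown without damage only when Indestruct is false, which BeginPlay sets shortly after spawn.
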(event OnComponentBeginOverlap(Box)
  (params (OverlappedComponent :type Primitive%20Component%20Object%20Reference) (OtherActor :type Actor%20Object%20Reference) (OtherComp :type Primitive%20Component%20Object%20Reference) (OtherBodyIndex :type Integer) (bFromSweep :type Boolean) (SweepResult :type Hit%20Result%20Structure%20%28by%20ref%29))
  (bind _pointlight (Variables|Default|GetPointLight))
  (bind _returnvalue (Transformation|GetWorldTransform _pointlight))
  (bind _asgrim_dig_pawn (Utilities|Casting|CastToGrimDigPawn OtherActor)
    (:then
      (if (not (Variables|/Game/Blueprints/Character/GrimDigPawn.GrimDigPawn_C|GetPlayerDead _asgrim_dig_pawn))
        (Game|Damage|ApplyDamage _asgrim_dig_pawn (Variables|Default|GetDamageRating) 0 0)
        (Components|Movement|StopMovementImmediately (Variables|Default|GetProjectileMovement) :!label _label)
        (Effects|Components|ParticleSystem|SetEmitterEnable (Variables|Default|GetParticleSystem) "FX_Fire" false)
        (Utilities|FlowControl|Sequence
          (:then_0
            (Utilities|FlowControl|Delay 1.0)
            (Actor|DestroyActor))
          (:then_1
            (Timeline|Timeline_0 Play
              (:Update
                (Rendering|Components|Light|SetIntensity (Variables|Default|GetPointLight) 0.0))))
          (:then_2
            (Effects|SpawnEmitteratLocation "/Game/Assets/ParticleFX/P_FX_SmokeRing.P_FX_SmokeRing" (.location _returnvalue) (.rotation _returnvalue) (.scale _returnvalue))))))
    (:CastFailed
      (if (not (Variables|Default|GetIndestruct))
        (goto _label)))))

(event EventBeginPlay
  (Utilities|FlowControl|Delay 0.2)
  (Variables|Default|SetIndestruct false))

(event Collision|EventActorBeginOverlap
  (params (OtherActor :type Actor%20Object%20Reference)))

(event EventTick
  (params (DeltaSeconds :type Float%20%28single-precision%29)))

(fn ConstructionScript)