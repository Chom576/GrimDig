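; BP_SpearTrap is an activable spike trap that damages the player pawn.
; TurnOn/Open, TurnOff/Close and the toggling Activate play or reverse a timeline that slides the spike mesh between start and end marker components.
; IsMoving blocks new commands mid-motion, and IsActive records the final state from the timeline direction.
; A box overlap applies fixed damage to any GrimDigPawn, without checking the trap's state.
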(event OnComponentBeginOverlap(Box)
  (params (OverlappedComponent :type Primitive%20Component%20Object%20Reference) (OtherActor :type Actor%20Object%20Reference) (OtherComp :type Primitive%20Component%20Object%20Reference) (OtherBodyIndex :type Integer) (bFromSweep :type Boolean) (SweepResult :type Hit%20Result%20Structure%20%28by%20ref%29))
  (bind _asgrim_dig_pawn (Utilities|Casting|CastToGrimDigPawn OtherActor))
  (Game|Damage|ApplyDamage _asgrim_dig_pawn 4e+01 0 0))

(event EventBeginPlay
  (|CallParentFunction) ; This node is disabled and will not be called.\nDrag off pins to build functionality.
)

(event Collision|EventActorBeginOverlap
  (params (OtherActor :type Actor%20Object%20Reference))
  (|CallParentFunction OtherActor) ; This node is disabled and will not be called.\nDrag off pins to build functionality.
)

(event EventTick
  (params (DeltaSeconds :type Float%20%28single-precision%29))
  (|CallParentFunction DeltaSeconds) ; This node is disabled and will not be called.\nDrag off pins to build functionality.
)

(event EventActivate
  (params (Initiator :type Actor%20Object%20Reference))
  (if (not (Variables|Default|GetIsMoving))
    (Variables|Default|SetIsMoving true)
    (if (Variables|Default|GetIsActive)
      (bind (_direction _newtrack_0) (Timeline|Timeline_0 ReverseFromEnd)
        (:Update
          (Transformation|SetRelativeLocation (Variables|Default|GetSM_Prop_Trap_Spikes_01) (Math|Vector|Lerp(Vector) (Variables|/Script/Engine.SceneComponent|GetRelativeLocation (Variables|Default|GetSpikeStart)) (Variables|/Script/Engine.SceneComponent|GetRelativeLocation (Variables|Default|GetSpikeEnd)) _newtrack_0) false false))
        (:Finished
          (Variables|Default|SetIsMoving false)
          (Variables|Default|SetIsActive (Utilities|Select :Index _direction :Forward true :Backward false))))
      (else
        (Timeline|Timeline_0 PlayFromStart)))))

(event EventTurnOff/Close
  (params (Initiator :type Actor%20Object%20Reference))
  (if (not (Variables|Default|GetIsMoving))
    (if (Variables|Default|GetIsActive)
      (Variables|Default|SetIsMoving true)
      (bind (_direction _newtrack_0) (Timeline|Timeline_0 ReverseFromEnd)
        (:Update
          (Transformation|SetRelativeLocation (Variables|Default|GetSM_Prop_Trap_Spikes_01) (Math|Vector|Lerp(Vector) (Variables|/Script/Engine.SceneComponent|GetRelativeLocation (Variables|Default|GetSpikeStart)) (Variables|/Script/Engine.SceneComponent|GetRelativeLocation (Variables|Default|GetSpikeEnd)) _newtrack_0) false false))
        (:Finished
          (Variables|Default|SetIsMoving false)
          (Variables|Default|SetIsActive (Utilities|Select :Index _direction :Forward true :Backward false)))))))

(event EventTurnOn/Open
  (params (Initiator :type Actor%20Object%20Reference))
  (if (not (Variables|Default|GetIsMoving))
    (if (not (Variables|Default|GetIsActive))
      (Variables|Default|SetIsMoving true)
      (bind (_direction _newtrack_0) (Timeline|Timeline_0 PlayFromStart)
        (:Update
          (Transformation|SetRelativeLocation (Variables|Default|GetSM_Prop_Trap_Spikes_01) (Math|Vector|Lerp(Vector) (Variables|/Script/Engine.SceneComponent|GetRelativeLocation (Variables|Default|GetSpikeStart)) (Variables|/Script/Engine.SceneComponent|GetRelativeLocation (Variables|Default|GetSpikeEnd)) _newtrack_0) false false))
        (:Finished
          (Variables|Default|SetIsMoving false)
          (Variables|Default|SetIsActive (Utilities|Select :Index _direction :Forward true :Backward false)))))))

(fn ConstructionScript
  (|CallParentFunction))