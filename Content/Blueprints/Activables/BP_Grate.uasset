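; Activatable grate that swings between open and closed, with an optional climbable tag and a configurable starting state.
; Activate, TurnOn and TurnOff drive a timeline that lerps the rotation between two reference components, ignoring calls while moving.
; Two overlap boxes track the player pawn above and below.
; Opening makes the lower player climb or get pushed; closing damages them and makes the upper player lose footing after a short delay.
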(event OnComponentBeginOverlap(BoxUp)
  (params (OverlappedComponent :type Primitive%20Component%20Object%20Reference) (OtherActor :type Actor%20Object%20Reference) (OtherComp :type Primitive%20Component%20Object%20Reference) (OtherBodyIndex :type Integer) (bFromSweep :type Boolean) (SweepResult :type Hit%20Result%20Structure%20%28by%20ref%29))
  (bind _asgrim_dig_pawn (Utilities|Casting|CastToGrimDigPawn OtherActor))
  (Variables|Default|SetPlayerRefUp _asgrim_dig_pawn))

(event OnComponentEndOverlap(BoxUp)
  (params (OverlappedComponent :type Primitive%20Component%20Object%20Reference) (OtherActor :type Actor%20Object%20Reference) (OtherComp :type Primitive%20Component%20Object%20Reference) (OtherBodyIndex :type Integer))
  (Utilities|Casting|CastToGrimDigPawn OtherActor)
  (Variables|Default|SetPlayerRefUp 0))

(event OnComponentBeginOverlap(BoxDown)
  (params (OverlappedComponent :type Primitive%20Component%20Object%20Reference) (OtherActor :type Actor%20Object%20Reference) (OtherComp :type Primitive%20Component%20Object%20Reference) (OtherBodyIndex :type Integer) (bFromSweep :type Boolean) (SweepResult :type Hit%20Result%20Structure%20%28by%20ref%29))
  (bind _asgrim_dig_pawn (Utilities|Casting|CastToGrimDigPawn OtherActor))
  (Variables|Default|SetPlayerRefDown _asgrim_dig_pawn))

(event OnComponentEndOverlap(BoxDown)
  (params (OverlappedComponent :type Primitive%20Component%20Object%20Reference) (OtherActor :type Actor%20Object%20Reference) (OtherComp :type Primitive%20Component%20Object%20Reference) (OtherBodyIndex :type Integer))
  (Utilities|Casting|CastToGrimDigPawn OtherActor)
  (Variables|Default|SetPlayerRefDown 0))

(event Custom|PlayerFalling?
  ;[1 1 1] Player Lost Footing
  (Default|EndMovement (Variables|Default|GetPlayerRefUp)))

(event EventBeginPlay
  (|CallParentFunction)
  (if (Variables|Default|GetClimbable)
    (Variables|Default|SetTags (Utilities|Array|MakeArray "Climbable")))
  (bind _output_get (Variables|Default|SetIsOpen (Variables|Default|GetStartOpen)))
  (if _output_get
    (Transformation|SetRelativeRotation (Variables|Default|GetScene) (Variables|/Script/Engine.SceneComponent|GetRelativeRotation (Variables|Default|GetOpen)) false false)
    (else
      (Transformation|SetRelativeRotation (Variables|Default|GetScene) (Variables|/Script/Engine.SceneComponent|GetRelativeRotation (Variables|Default|GetClosed)) false false))))

(event Collision|EventActorBeginOverlap
  (params (OtherActor :type Actor%20Object%20Reference))
  (|CallParentFunction OtherActor) ; This node is disabled and will not be called.\nDrag off pins to build functionality.
)

(event EventTick
  (params (DeltaSeconds :type Float%20%28single-precision%29))
  (|CallParentFunction DeltaSeconds) ; This node is disabled and will not be called.\nDrag off pins to build functionality.
)

(event EventActivate
  (params (Initiator :type Actor%20Object%20Reference))
  (bind _playerrefdown (Variables|Default|GetPlayerRefDown))
  (bind _playerrefup (Variables|Default|GetPlayerRefUp))
  (bind _playerrefdown_2 (Variables|Default|GetPlayerRefDown))
  (bind _playerrefdown_3 (Variables|Default|GetPlayerRefDown))
  (if (not (Variables|Default|GetIsMoving))
    (if (Variables|Default|GetIsOpen)
      (Variables|Default|SetIsMoving true)
      ;[1 1 1] Player Lost Footing
      (Utilities|IsValid _playerrefup
        (:Is%20Valid
          (Variables|/Game/Blueprints/Character/GrimDigPawn.GrimDigPawn_C|SetMovementInProgress _playerrefup true)
          (Utilities|Time|SetTimerbyEvent (delegate Custom|PlayerFalling?) 0.3))
        (:Is%20Not%20Valid
          _))
      ;[1 1 1] PlayerCrushed
      (Utilities|IsValid _playerrefdown
        (:Is%20Valid
          (Game|Damage|ApplyDamage _playerrefdown 1e+02 0 0)
          (bind (_direction _newtrack_0) (Timeline|Timeline_0 ReverseFromEnd)
            (:Update
              (Transformation|SetRelativeRotation (Variables|Default|GetScene) (Math|Rotator|Lerp(Rotator) (Variables|/Script/Engine.SceneComponent|GetRelativeRotation (Variables|Default|GetClosed)) (Variables|/Script/Engine.SceneComponent|GetRelativeRotation (Variables|Default|GetOpen)) _newtrack_0) false false))
            (:Finished
              (Variables|Default|SetIsMoving false)
              (Variables|Default|SetIsOpen (Utilities|Select :Index _direction :Forward true :Backward false)))))
        (:Is%20Not%20Valid
          (Timeline|Timeline_0 ReverseFromEnd)))
      (else
        (Variables|Default|SetIsMoving true)
        (Utilities|IsValid _playerrefdown_2
          (:Is%20Valid
            (Variables|/Game/Blueprints/Character/GrimDigPawn.GrimDigPawn_C|SetMovementInProgress _playerrefdown_2 true)
            (if (Variables|/Game/Blueprints/Character/GrimDigPawn.GrimDigPawn_C|GetIsClimbing _playerrefdown_2)
              ;[1 1 1] Player Climbs
              (Variables|/Game/Blueprints/Character/GrimDigPawn.GrimDigPawn_C|SetScheduledActions (Variables|Default|GetPlayerRefDown) (Utilities|Array|MakeArray "NewEnumerator4" "NewEnumerator6"))
              (else
                ;[1 1 1] Player Pushed
                (Variables|/Game/Blueprints/Character/GrimDigPawn.GrimDigPawn_C|SetForcedMoveVector _playerrefdown_3 (Math|Vector|Normalize (- (Transformation|GetWorldLocation (Variables|Default|GetEndMovement)) (Transformation|GetActorLocation (Variables|Default|GetPlayerRefDown)))))
                (Variables|/Game/Blueprints/Character/GrimDigPawn.GrimDigPawn_C|SetScheduledActions _playerrefdown_3 (Utilities|Array|MakeArray "NewEnumerator16"))))
            (Default|EndMovement (Variables|Default|GetPlayerRefDown))
            (Timeline|Timeline_0 PlayFromStart))
          (:Is%20Not%20Valid
            (Timeline|Timeline_0 PlayFromStart)))))))

(event EventTurnOff/Close
  (params (Initiator :type Actor%20Object%20Reference))
  (bind _playerrefdown (Variables|Default|GetPlayerRefDown))
  (bind _playerrefup (Variables|Default|GetPlayerRefUp))
  (if (not (Variables|Default|GetIsMoving))
    (if (Variables|Default|GetIsOpen)
      (Variables|Default|SetIsMoving true)
      ;[1 1 1] Player Lost Footing
      (Utilities|IsValid _playerrefup
        (:Is%20Valid
          (Variables|/Game/Blueprints/Character/GrimDigPawn.GrimDigPawn_C|SetMovementInProgress _playerrefup true)
          (Utilities|Time|SetTimerbyEvent (delegate Custom|PlayerFalling?) 0.3))
        (:Is%20Not%20Valid
          _))
      ;[1 1 1] PlayerCrushed
      (Utilities|IsValid _playerrefdown
        (:Is%20Valid
          (Game|Damage|ApplyDamage _playerrefdown 1e+02 0 0)
          (bind (_direction _newtrack_0) (Timeline|Timeline_0 ReverseFromEnd)
            (:Update
              (Transformation|SetRelativeRotation (Variables|Default|GetScene) (Math|Rotator|Lerp(Rotator) (Variables|/Script/Engine.SceneComponent|GetRelativeRotation (Variables|Default|GetClosed)) (Variables|/Script/Engine.SceneComponent|GetRelativeRotation (Variables|Default|GetOpen)) _newtrack_0) false false))
            (:Finished
              (Variables|Default|SetIsMoving false)
              (Variables|Default|SetIsOpen (Utilities|Select :Index _direction :Forward true :Backward false)))))
        (:Is%20Not%20Valid
          (Timeline|Timeline_0 ReverseFromEnd))))))

(event EventTurnOn/Open
  (params (Initiator :type Actor%20Object%20Reference))
  (bind _playerrefdown (Variables|Default|GetPlayerRefDown))
  (bind _playerrefdown_2 (Variables|Default|GetPlayerRefDown))
  (if (not (Variables|Default|GetIsMoving))
    (if (not (Variables|Default|GetIsOpen))
      (Variables|Default|SetIsMoving true)
      (Utilities|IsValid _playerrefdown
        (:Is%20Valid
          (Variables|/Game/Blueprints/Character/GrimDigPawn.GrimDigPawn_C|SetMovementInProgress _playerrefdown true)
          (if (Variables|/Game/Blueprints/Character/GrimDigPawn.GrimDigPawn_C|GetIsClimbing _playerrefdown)
            ;[1 1 1] Player Climbs
            (Variables|/Game/Blueprints/Character/GrimDigPawn.GrimDigPawn_C|SetScheduledActions (Variables|Default|GetPlayerRefDown) (Utilities|Array|MakeArray "NewEnumerator4" "NewEnumerator6"))
            (else
              ;[1 1 1] Player Pushed
              (Variables|/Game/Blueprints/Character/GrimDigPawn.GrimDigPawn_C|SetForcedMoveVector _playerrefdown_2 (Math|Vector|Normalize (- (Transformation|GetWorldLocation (Variables|Default|GetEndMovement)) (Transformation|GetActorLocation (Variables|Default|GetPlayerRefDown)))))
              (Variables|/Game/Blueprints/Character/GrimDigPawn.GrimDigPawn_C|SetScheduledActions _playerrefdown_2 (Utilities|Array|MakeArray "NewEnumerator16"))))
          (Default|EndMovement (Variables|Default|GetPlayerRefDown))
          (bind (_direction _newtrack_0) (Timeline|Timeline_0 PlayFromStart)
            (:Update
              (Transformation|SetRelativeRotation (Variables|Default|GetScene) (Math|Rotator|Lerp(Rotator) (Variables|/Script/Engine.SceneComponent|GetRelativeRotation (Variables|Default|GetClosed)) (Variables|/Script/Engine.SceneComponent|GetRelativeRotation (Variables|Default|GetOpen)) _newtrack_0) false false))
            (:Finished
              (Variables|Default|SetIsMoving false)
              (Variables|Default|SetIsOpen (Utilities|Select :Index _direction :Forward true :Backward false)))))
        (:Is%20Not%20Valid
          (Timeline|Timeline_0 PlayFromStart))))))

(fn ConstructionScript
  (|CallParentFunction)
  (bind _output_get (Variables|Default|SetIsOpen (Variables|Default|GetStartOpen)))
  (if _output_get
    (Transformation|SetRelativeRotation (Variables|Default|GetScene) (Variables|/Script/Engine.SceneComponent|GetRelativeRotation (Variables|Default|GetOpen)) false false)
    (else
      (Transformation|SetRelativeRotation (Variables|Default|GetScene) (Variables|/Script/Engine.SceneComponent|GetRelativeRotation (Variables|Default|GetClosed)) false false))))